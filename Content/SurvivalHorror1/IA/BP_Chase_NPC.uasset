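; BP_Chase_NPC is the survival horror chaser NPC that reacts to touching the player and can be stunned.
; Its collision overlap casts to BP_MainCharacter and calls IATouchMessage through a DoOnce, which has no reset here.
; Stun sets a Blackboard bool and StunState, then disables collision overlap events for a fixed delay.
; Afterwards it restores StunState and overlaps but leaves the Blackboard bool set.
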(event `self.ReceiveBeginPlay`)

(event `/Game/SurvivalHorror1/Blueprints/Main_Character/BPI_Stun.Stun`
  (`KismetSystemLibrary.PrintString` "Aille! (bot stun)")
  (`BlackboardComponent.SetValueAsBool` (`AIBlueprintHelperLibrary.GetBlackboard` null) (`self.Key Name`) true)
  (set `self.stunState` true)
  (set `PrimitiveComponent.bGenerateOverlapEvents` false (`self.collision`))
  (`KismetSystemLibrary.Delay` 15.0)
  (set `self.stunState` false)
  (set `PrimitiveComponent.bGenerateOverlapEvents` true (`self.collision`)))

(event `self.collision.OnComponentBeginOverlap`
  (params (OverlappedComponent :type "PrimitiveComponent Object Reference") (OtherActor :type "Actor Object Reference") (OtherComp :type "PrimitiveComponent Object Reference") (OtherBodyIndex :type Integer) (bFromSweep :type Boolean) (SweepResult :type "HitResult Structure (by ref)"))
  (bind _asbp_main_character (cast `/Game/SurvivalHorror1/Blueprints/Main_Character/BP_MainCharacter` OtherActor))
  (`/Engine/EditorBlueprintResources/StandardMacros.DoOnce` false
    (:`Completed`
      (message `/Game/SurvivalHorror1/IA/BPI_IA.IATouch` _asbp_main_character))))

(fn `UserConstructionScript`)