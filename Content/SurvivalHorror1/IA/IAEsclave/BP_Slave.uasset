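; BP_Slave is an AI-controlled slave character that can grab the player in a survival horror game.
; While alive, its Capsule overlap calls SlavegrabMessage on BP_MainCharacter.
; Overlapping a BP_Chase_NPC disables collision for three seconds on a mesh constraint, looked up by the capsule's collision profile name.
; Stun calls EventKill on its AI controller, enables capsule physics and marks it dead.
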(event `self.Capsule.OnComponentBeginOverlap`
  (params (OverlappedComponent :type "PrimitiveComponent Object Reference") (OtherActor :type "Actor Object Reference") (OtherComp :type "PrimitiveComponent Object Reference") (OtherBodyIndex :type Integer) (bFromSweep :type Boolean) (SweepResult :type "HitResult Structure (by ref)"))
  (bind _mesh (`self.Mesh`))
  (bind _returnvalue (`PrimitiveComponent.GetCollisionProfileName` (`self.CapsuleComponent`)))
  (bind _asbp_main_character (cast `/Game/SurvivalHorror1/Blueprints/Main_Character/BP_MainCharacter` OtherActor)
    (:`then`
      (if (not (`self.Isdead`))
        (message `/Game/SurvivalHorror1/IA/IAEsclave/BPI_Slavetouch.Slavegrab` _asbp_main_character)))
    (:`CastFailed`
      (cast `/Game/SurvivalHorror1/IA/BP_Chase_NPC` OtherActor)
      (bind _outactors (`GameplayStatics.GetAllActorsOfClass` "/Game/SurvivalHorror1/IA/BP_Chase_NPC.BP_Chase_NPC_C"))
      (cast `/Game/SurvivalHorror1/IA/BP_Chase_NPC` (`|GetArrayItem` _outactors))
      (bind _returnvalue_2 (`SkeletalMeshComponent.GetConstraintByName` _mesh _returnvalue false))
      (`ConstraintInstanceBlueprintLibrary.SetDisableCollision` _returnvalue_2 true)
      (`KismetSystemLibrary.Delay` 3.0)
      (bind _returnvalue_3 (`SkeletalMeshComponent.GetConstraintByName` _mesh _returnvalue false))
      (`ConstraintInstanceBlueprintLibrary.SetDisableCollision` _returnvalue_3))))

(event `/Game/SurvivalHorror1/Blueprints/Main_Character/BPI_Stun.Stun`
  (bind _asbp_slave_ai_controller (cast `/Game/SurvivalHorror1/IA/IAEsclave/BP_SlaveAI_Controller` (`self.GetController`)))
  (`/Game/SurvivalHorror1/IA/IAEsclave/BP_SlaveAI_Controller.Event Kill` _asbp_slave_ai_controller)
  (`PrimitiveComponent.SetSimulatePhysics` (`self.CapsuleComponent`) true)
  (set `self.Isdead` true))

(fn `UserConstructionScript`)