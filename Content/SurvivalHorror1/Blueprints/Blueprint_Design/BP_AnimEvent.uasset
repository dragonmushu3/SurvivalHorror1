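; BP_AnimEvent is a one-shot trigger that plays a spawned skeletal mesh animation when BP_MainCharacter overlaps it.
; It spawns a BP_SkeletalMeshActor offset from the trigger, applies the configured rotation, mesh and physics-only collision, then plays the animation with an optional sound.
; The spawned actor is destroyed after the animation's length.
; A DoOnce prevents repeats, resetting only when the overlapping actor is not the main character.
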(event `self.ReceiveActorBeginOverlap`
  (params (OtherActor :type "Actor Object Reference"))
  (bind _soundtoplay (`self.SoundToPlay`))
  (bind _animationtoplay (`self.AnimationToPlay`))
  (bind _spawnpoint_location (`KismetMathLibrary.BreakTransform` (`self.SpawnPoint`)))
  (`/Engine/EditorBlueprintResources/StandardMacros.DoOnce` false :!label _label
    (:`Completed`
      (bind _asbp_main_character (cast `/Game/SurvivalHorror1/Blueprints/Main_Character/BP_MainCharacter` OtherActor)
        (:`then`
          (`/Engine/EditorBlueprintResources/StandardMacros.IsValid` _asbp_main_character
            (:`Is Valid`
              (bind _output_get (set `self.SpawnPoint` (`KismetMathLibrary.MakeTransform` (+ (.location (`self.GetTransform`)) (.location (`self.SpawnLocation`))) (struct) (.scale (`self.SpawnLocation`)))))
              (bind _returnvalue (`|SpawnActorFromClass` "/Game/SurvivalHorror1/Blueprints/Blueprint_Design/BP_SkeletalMeshActor.BP_SkeletalMeshActor_C" _output_get "AdjustIfPossibleButAlwaysSpawn" "OverrideRootScale" null null))
              (`self.K2_SetActorRotation` _returnvalue (.rotation (`self.SpawnLocation`)) false)
              (bind _skeletalmesh (`/Game/SurvivalHorror1/Blueprints/Blueprint_Design/BP_SkeletalMeshActor.SkeletalMesh` _returnvalue))
              (`PrimitiveComponent.SetCollisionEnabled` _skeletalmesh "PhysicsOnly")
              (`SkeletalMeshComponent.SetSkeletalMeshAsset` _skeletalmesh (`self.Mesh`))
              (`SkeletalMeshComponent.PlayAnimation` _skeletalmesh _animationtoplay false)
              (if (`KismetSystemLibrary.IsValid` _soundtoplay)
                (`GameplayStatics.PlaySoundAtLocation` _soundtoplay _spawnpoint_location (struct) 1.0 1.0 0.0 null null null null))
              (`KismetSystemLibrary.Delay` (`AnimSequenceBase.SequenceLength` _animationtoplay))
              (`self.K2_DestroyActor` _returnvalue))
            (:`Is Not Valid`
              (goto _label :!via `Reset`))))
        (:`CastFailed`
          (goto _label :!via `Reset`))))))

(fn `UserConstructionScript`)