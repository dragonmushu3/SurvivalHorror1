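; DoorLinkBP is a door whose OpenDoor event toggles it between open and closed.
; A timeline plays or reverses to swing the door mesh's relative yaw through a quarter turn.
; When the timeline finishes, a short delay precedes switching the first player's view target to the actor passed into the event and restoring game-only input.
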(event `Open Door`
  (params (InputPin :type "Actor Object Reference"))
  (bind _returnvalue (`GameplayStatics.GetPlayerController` 0))
  (bind _output_get (set `self.Openning?` (not (`self.Openning?`))))
  (if _output_get
    (bind (_direction _door) (`Timeline|Open/Close Door` :!label _label)
      (:`Update`
        (`SceneComponent.K2_SetRelativeRotation` (`self.SM_Door`) (`KismetMathLibrary.MakeRotator` 0.0 0.0 (`KismetMathLibrary.Lerp` 0.0 90.0 _door)) false false))
      (:`Finished`
        (`KismetSystemLibrary.Delay` 1.0)
        (`PlayerController.SetViewTargetWithBlend` _returnvalue InputPin 0.0 "VTBlend_Linear" 0.0 false)
        (`WidgetBlueprintLibrary.SetInputMode_GameOnly` _returnvalue)))
    (else
      (goto _label :!via `Reverse`))))

(fn `UserConstructionScript`)