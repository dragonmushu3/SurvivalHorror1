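; Interactable wall or door button that remotely opens the DoorLinkBP door sharing its ButtonValue.
; Each interaction toggles a Timeline forward or backward to slide the button's Cube along X.
; It also searches all DoorLinkBP actors for the first matching DoorValue and calls OpenDoor with the player.
; The camera then blends to that door and input switches to UI only.
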(event `/Game/SurvivalHorror1/Blueprints/Main_Character/BPI_Interact.Interact`
  (params (Player :type "/Game/SurvivalHorror1/Blueprints/Main_Character/BP_MainCharacter Object Reference"))
  (bind _returnvalue (`GameplayStatics.GetPlayerController` 0))
  (`|ExecutionSequence`
    (:`then_0`
      (`/Engine/EditorBlueprintResources/StandardMacros.FlipFlop`
        (:`A`
          (bind (_direction _newtrack_0) (`Timeline|Timeline` :!label _label)
            (:`Update`
              (`SceneComponent.K2_SetRelativeLocation` (`self.Cube`) (`KismetMathLibrary.MakeVector` (* (`KismetMathLibrary.Lerp` 0.0 4.0 _newtrack_0) -1.0)) false false))))
        (:`B`
          (goto _label :!via `Reverse`))))
    (:`then_1`
      (bind _outactors (`GameplayStatics.GetAllActorsOfClass` "/Game/SurvivalHorror1/Blueprints/Items/Door/DoorLinkBP.DoorLinkBP_C"))
      (for _array_element _outactors
        (if (== (`/Game/SurvivalHorror1/Blueprints/Items/Door/DoorLinkBP.DoorValue` _array_element) (`self.ButtonValue`))
          (if (`self.Do Once`)
            (`/Engine/EditorBlueprintResources/StandardMacros.DoOnce` false
              (:`Completed`
                _)))
          (`/Game/SurvivalHorror1/Blueprints/Items/Door/DoorLinkBP.Open Door` _array_element Player)
          (`PlayerController.SetViewTargetWithBlend` _returnvalue _array_element 0.0 "VTBlend_Linear" 0.0 false)
          (`WidgetBlueprintLibrary.SetInputMode_UIOnlyEx` _returnvalue null "LockInFullscreen")
          (break))))))

(fn `UserConstructionScript`)