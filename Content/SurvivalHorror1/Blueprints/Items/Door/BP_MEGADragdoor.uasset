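; BP_MEGADragdoor is a door the player drags open or shut by holding left mouse while looking at it.
; On press, a debug-drawn line trace from the BP_MainCharacter camera sets a looking flag when it hits any door of this class.
; While held, Tick adds the character's TurnRate as local yaw to the Door, with no clamping or delta-time scaling.
; Each door enables its own input on BeginPlay.
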(event `self.ReceiveTick`
  (params (DeltaSeconds :type "Float (single-precision)"))
  (if (`self.isHoldingLMB?`)
    (if (`self.isLookingAtDoor?`)
      (if true
        (`SceneComponent.K2_AddLocalRotation` (`self.Door`) (`KismetMathLibrary.MakeRotator` 0.0 0.0 (`/Game/SurvivalHorror1/Blueprints/Main_Character/BP_MainCharacter.Turn Rate` (stale `Key|LeftMouseButton` _asbp_main_character))) false false)))))

(event `self.ReceiveBeginPlay`
  (`self.EnableInput` (`GameplayStatics.GetPlayerController` 0)))

(event `Key|LeftMouseButton`
  (params (Key :type "Key Structure"))
  (:`Pressed`
    (set `self.isHoldingLMB?` true)
    (bind _asbp_main_character (cast `/Game/SurvivalHorror1/Blueprints/Main_Character/BP_MainCharacter` (`GameplayStatics.GetPlayerCharacter` 0)))
    (bind _cameracomp (`MainCharacter.CameraComp` _asbp_main_character))
    (bind _returnvalue (`SceneComponent.K2_GetComponentLocation` _cameracomp))
    (bind (_outhit _returnvalue_2) (`KismetSystemLibrary.LineTraceSingleForObjects` :`Start` _returnvalue :`End` (+ _returnvalue (* (`SceneComponent.GetForwardVector` _cameracomp) 500.0)) :`ObjectTypes` (`|MakeArray` "ObjectTypeQuery2" :!type "EObjectTypeQuery Enum") :`DrawDebugType` "ForDuration"))
    (if _returnvalue_2
      (cast `/Game/SurvivalHorror1/Blueprints/Items/Door/BP_MEGADragdoor` (`.HitActor` (`GameplayStatics.BreakHitResult` _outhit)))
      (set `self.isLookingAtDoor?` true)
      (else
        (set `self.isLookingAtDoor?` false))))
  (:`Released`
    (set `self.isHoldingLMB?` false)))

(fn `UserConstructionScript`)