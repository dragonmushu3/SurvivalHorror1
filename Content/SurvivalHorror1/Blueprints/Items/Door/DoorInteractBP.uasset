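; Interactable door Blueprint for a survival horror game that swings open and closed, optionally gated by power and a key.
; Interact calls OpenDoor, which checks the power state set by IsPowered, then searches the player's inventory component for a matching key value when one is required.
; Each successful check toggles the open state and plays or reverses a timeline that lerps the door mesh's relative yaw.
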(event `/Game/SurvivalHorror1/Blueprints/Main_Character/BPI_Interact.Interact`
  (params (Player :type "/Game/SurvivalHorror1/Blueprints/Main_Character/BP_MainCharacter Object Reference"))
  (`self.Open Door` Player))

(event `/Game/SurvivalHorror1/Blueprints/Furniture/BPI_Power.isPowered`
  (params (`PowerOn?` :type Boolean))
  (set `self.Power?` `PowerOn?`))

(event `Open Door`
  (params (REF :type "/Game/SurvivalHorror1/Blueprints/Main_Character/BP_MainCharacter Object Reference"))
  (if (`self.PowerNeeded?`)
    (if (`self.Power?`)
      (if (`self.KeyNeeded?`) :!label _label
        (for _array_element (`/Game/SurvivalHorror1/Blueprints/Inventory_V2/Comp_Inventory.Inventory` (`/Game/SurvivalHorror1/Blueprints/Main_Character/BP_MainCharacter.Comp_Inventory` REF))
          (if (`KismetTextLibrary.EqualEqual_TextText` (`self.KeyValue`) (`.Value_19_73967ECD4B84F205A44C5F98B143AD1A` (break `/Game/SurvivalHorror1/Blueprints/Inventory_V2/ST_Inventory` _array_element)))
            (if (`self.Do Once`) :!label _label_2
              (`/Engine/EditorBlueprintResources/StandardMacros.DoOnce` false
                (:`Completed`
                  _)))
            (bind _output_get (set `self.Openning?` (not (`self.Openning?`))))
            (if _output_get
              (bind (_direction _door) (`Timeline|Open/Close Door` :!label _label_3)
                (:`Update`
                  (`SceneComponent.K2_SetRelativeRotation` (`self.SM_Door`) (`KismetMathLibrary.MakeRotator` 0.0 0.0 (`KismetMathLibrary.Lerp` 0.0 90.0 _door)) false false)))
              (else
                (goto _label_3 :!via `Reverse`)))))
        (else
          (goto _label_2))))
    (else
      (goto _label))))

(fn `UserConstructionScript`)