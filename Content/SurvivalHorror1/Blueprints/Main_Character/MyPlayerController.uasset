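; Player controller that manages the player's gameplay ability hotbar, keeping the ability array and HUD button icons in step.
; On BeginPlay it caches the main character, whose HUD reference leads to the hotbar buttons.
; Helpers check for free space, place picked-up abilities in the first empty slot and set that button's icon.
; Separate move functions swap or move abilities and images between slots, linked by a Swapping flag.
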(event `self.ReceiveBeginPlay`
  (bind _asbp_main_character (cast `/Game/SurvivalHorror1/Blueprints/Main_Character/BP_MainCharacter` (`GameplayStatics.GetPlayerCharacter` 0)))
  (set `self.CharacterREF` _asbp_main_character))

(fn `FindEmptyHotbarSlot`
  (returns (Index :type Integer))
  (for (_array_element _array_index) (`self.GameplayAbilityHotbar`)
    (if (not (`KismetSystemLibrary.IsValid` _array_element))
      (set `self.EmptyHotbarSlot` _array_index)
      (break)))
  (return (`self.EmptyHotbarSlot`)))

(fn `HotbarCheck`
  (returns (`HasSpace?` :type Boolean))
  (for _array_element (`self.GameplayAbilityHotbar`)
    (if (`KismetSystemLibrary.IsValid` _array_element)
      (set `self.HasHotbarSpace?` false)
      (else
        (set `self.HasHotbarSpace?` true)
        (break))))
  (return (`self.HasHotbarSpace?`)))

(fn `MoveAbilityWithinHotbar`
  (params (From :type Integer) (To :type Integer))
  (returns (`Swapping?` :type Boolean))
  (locals (LocalFrom :type Integer) (LoacalTo :type Integer) (`LocalSwapping?` :type Boolean) (LocalTemporaryGameplayAbility :type "/Game/SurvivalHorror1/Blueprints/GameplayAbilities/GameplayAbility Object Reference"))
  (set `local.LocalFrom` From)
  (set `local.LoacalTo` To)
  (if (`KismetArrayLibrary.Array_IsValidIndex` (`self.GameplayAbilityHotbar`) (`local.LoacalTo`))
    (set `local.LocalTemporaryGameplayAbility` (`|GetArrayItem` (`self.GameplayAbilityHotbar`) (`local.LoacalTo`)))
    (`KismetArrayLibrary.Array_Set` (`self.GameplayAbilityHotbar`) (`local.LoacalTo`) (`|GetArrayItem` (`self.GameplayAbilityHotbar`) (`local.LocalFrom`)))
    (`KismetArrayLibrary.Array_Set` (`self.GameplayAbilityHotbar`) (`local.LocalFrom`) (`local.LocalTemporaryGameplayAbility`))
    (set `local.LocalSwapping?` true)
    (else
      (`KismetArrayLibrary.Array_Set` (`self.GameplayAbilityHotbar`) (`local.LoacalTo`) (`|GetArrayItem` (`self.GameplayAbilityHotbar`) (`local.LocalFrom`)))
      (`KismetArrayLibrary.Array_Set` (`self.GameplayAbilityHotbar`) (`local.LocalFrom`))
      (set `local.LocalSwapping?` false)))
  (return (`local.LocalSwapping?`)))

(fn `MoveImageWithinHotbar`
  (params (From :type Integer) (To :type Integer) (AbilityImage :type "Texture2D Object Reference") (`Swapping?` :type Boolean))
  (locals (LocalFrom :type Integer) (LocalTo :type Integer) (LocalAbilityImage :type "Texture2D Object Reference") (LocalTeporaryAbilityImage :type "Texture2D Object Reference"))
  (bind _hotbarbuttons (`self.Hotbar Buttons Reference`))
  (bind _output (`|GetArrayItem` (`self.Hotbar Buttons Reference`) (`local.LocalTo`)))
  (set `local.LocalFrom` From)
  (set `local.LocalTo` To)
  (set `local.LocalAbilityImage` AbilityImage)
  (if `Swapping?`
    (set `local.LocalTeporaryAbilityImage` (`/Game/SurvivalHorror1/Blueprints/HotBar/HotbarSlot.AbilityImage` _output))
    (set `/Game/SurvivalHorror1/Blueprints/HotBar/HotbarSlot.AbilityImage` (`local.LocalAbilityImage`) _output)
    (set `/Game/SurvivalHorror1/Blueprints/HotBar/HotbarSlot.AbilityImage` (`local.LocalTeporaryAbilityImage`) (`|GetArrayItem` (`self.Hotbar Buttons Reference`) (`local.LocalFrom`)))
    (else
      (set `/Game/SurvivalHorror1/Blueprints/HotBar/HotbarSlot.AbilityImage` (`local.LocalAbilityImage`) (`|GetArrayItem` _hotbarbuttons (`local.LocalTo`)))
      (set `/Game/SurvivalHorror1/Blueprints/HotBar/HotbarSlot.AbilityImage` null (`|GetArrayItem` _hotbarbuttons (`local.LocalFrom`))))))

(fn `PickupAbility`
  (params (GameplayAbilityToPickUp :type "/Game/SurvivalHorror1/Blueprints/GameplayAbilities/GameplayAbility Object Reference"))
  (bind _output (`|GetArrayItem` (`self.Hotbar Buttons Reference`) (`self.EmptyHotbarSlot`)))
  (`KismetArrayLibrary.Array_Set` (`self.GameplayAbilityHotbar`) (`self.FindEmptyHotbarSlot`) GameplayAbilityToPickUp)
  (set `/Game/SurvivalHorror1/Blueprints/HotBar/HotbarSlot.AbilityImage` (`/Game/SurvivalHorror1/Blueprints/GameplayAbilities/GameplayAbility.GameplayAbilityIcon` GameplayAbilityToPickUp) _output)
  (`/Game/SurvivalHorror1/Blueprints/HotBar/HotbarSlot.SetButtonStyle` _output))

(fn `UserConstructionScript`)