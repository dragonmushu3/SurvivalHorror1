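; BP_ModularWall is a construction-script tool that builds a modular wall with connectors and random decorations.
; It divides the Y distance of LastInstanceEnd by the wall mesh's width to get the module count.
; Each module adds wall and connector instances along local negative Y to two instanced mesh groups.
; A random stream then scatters a few decoration meshes per module as separate components, positioned from the wall mesh's bounds.
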(fn `AddDecorations`
  (params (ModuleTransform :type "Transform Structure") (MeshLength :type "Float (double-precision)") (Index :type Integer))
  (bind _output_get (set `self.DeacorationCount` (`KismetMathLibrary.RandomIntegerInRangeFromStream` 0 3 (`self.RandomStream`))))
  (for _ (range _output_get)
    (bind _returnvalue (`self.Get Random Point Within Module` ModuleTransform (`self.MeshConnector`)))
    (bind _returnvalue_2 (`AddComponent|NODE_AddStaticMeshComponent-0` :`RelativeTransform` (`KismetMathLibrary.MakeTransform` (`KismetMathLibrary.MakeVector` 0.0 (* (.y _returnvalue) -1.0) (.z _returnvalue)))))
    (bind _output (`self.Get Random DecorationMesh`))
    (`StaticMeshComponent.SetStaticMesh` _returnvalue_2 _output)))

(fn `AddModule`
  (params (`Instance Index` :type Integer) (MeshLength :type "Float (double-precision)"))
  (returns (Index :type Integer) (Transform :type "Transform Structure"))
  (bind (_connectortransform_location _connectortransform_rotation _connectortransform_scale) (`KismetMathLibrary.BreakTransform` (`self.ConnectorTransform`)))
  (bind _returnvalue (`KismetMathLibrary.MakeTransform` (`KismetMathLibrary.MakeVector` 0.0 (* (* MeshLength `Instance Index`) -1.0)) (struct) (1.0 1.0 1.0)))
  (bind _returnvalue_2 (`KismetMathLibrary.MakeTransform` (+ _connectortransform_location (.location _returnvalue)) (struct) _connectortransform_scale))
  (`InstancedStaticMeshComponent.AddInstance` (`self.InstanceGroupWall`) _returnvalue false)
  (bind _returnvalue_3 (`InstancedStaticMeshComponent.AddInstance` (`self.InstanceGroupConnector`) _returnvalue_2 false))
  (return _returnvalue_3 _returnvalue_2))

(fn `CalcDistanceToEnd`
  (returns (ReturnValue :type "Float (double-precision)"))
  (bind (_lastinstanceend_x _lastinstanceend_y) (`KismetMathLibrary.BreakVector` (`self.LastInstanceEnd`)))
  (return (`KismetMathLibrary.FMax` _lastinstanceend_y 1.0)))

(fn `CalcInstanceCount`
  (params (DistanceToEnd :type "Float (double-precision)") (MeshLength :type "Float (double-precision)"))
  (returns (InstanceCount :type Integer))
  (return (`KismetMathLibrary.FFloor` (/ DistanceToEnd MeshLength))))

(fn `CalcMeshLength`
  (returns (ReturnValue :type "Float (double-precision)"))
  (bind (_returnvalue_origin _returnvalue_boxextent) (`KismetMathLibrary.BreakBoxSphereBounds` (`StaticMesh.GetBounds` (`self.MeshModule`))))
  (return (* (.y _returnvalue_boxextent) 2.0)))

(fn `Get Random DecorationMesh`
  (returns (Output :type "StaticMesh Object Reference"))
  (bind _decorationmeshes (`self.DecorationMeshes`))
  (return (`|GetArrayItem` _decorationmeshes (- (`KismetMathLibrary.RandomIntegerInRangeFromStream` 1 (`KismetArrayLibrary.Array_Length` _decorationmeshes) (`self.RandomStream`)) 1))))

(fn `Get Random Point Within Module`
  (params (T :type "Transform Structure (by ref)") (Target :type "StaticMesh Object Reference"))
  (returns (ReturnValue :type "Vector Structure"))
  (locals (RandomX :type "Float (single-precision)" :default 0.0) (RandomZ :type "Float (single-precision)" :default 0.0))
  (bind _returnvalue (`StaticMesh.GetBounds` (`self.MeshModule`)))
  (bind _returnvalue_2 (`KismetMathLibrary.MakeVector` (.x (`.BoxExtent` (`KismetMathLibrary.BreakBoxSphereBounds` _returnvalue))) (.y (`.BoxExtent` (`KismetMathLibrary.BreakBoxSphereBounds` _returnvalue))) (.z (`.BoxExtent` (`KismetMathLibrary.BreakBoxSphereBounds` _returnvalue)))))
  (`|ExecutionSequence`
    (:`then_0`
      (set `local.RandomX` (`KismetMathLibrary.RandomFloatInRangeFromStream` -1.0 1.0 (`self.RandomStream`))))
    (:`then_1`
      (set `local.RandomZ` (`KismetMathLibrary.RandomFloatInRangeFromStream` -1.0 1.0 (`self.RandomStream`))))
    (:`then_2`
      (`KismetSystemLibrary.PrintString` (`KismetStringLibrary.Conv_VectorToString` _returnvalue_2))
      (return (`KismetMathLibrary.TransformLocation` T (+ (* (`KismetMathLibrary.MakeVector` 0.0 (`local.RandomX`) (`local.RandomZ`)) _returnvalue_2) _returnvalue_2))))))

(fn `Initialize`
  (`StaticMeshComponent.SetStaticMesh` (`self.InstanceGroupWall`) (`self.MeshModule`))
  (`StaticMeshComponent.SetStaticMesh` (`self.InstanceGroupConnector`) (`self.MeshConnector`)))

(fn `UserConstructionScript`
  (locals (MeshLength :type "Float (double-precision)") (DistanceToEnd :type "Float (double-precision)"))
  (`|ExecutionSequence`
    (:`then_0`
      (`self.Initialize`))
    (:`then_1`
      (set `local.MeshLength` (`self.CalcMeshLength`)))
    (:`then_2`
      (set `local.DistanceToEnd` (`self.CalcDistanceToEnd`)))
    (:`then_3`
      (bind _instancecount (`self.CalcInstanceCount` (`local.DistanceToEnd`) (`local.MeshLength`)))
      (set `self.InstanceCount` _instancecount))
    (:`then_4`
      (for _index (range (`self.InstanceCount`))
        (bind (_index_2 _transform) (`self.AddModule` _index (`local.MeshLength`)))
        (`self.AddDecorations` _transform (`local.MeshLength`) _index)))))