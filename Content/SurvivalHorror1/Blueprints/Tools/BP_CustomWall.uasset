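; Modular wall tool that rebuilds a chain of static mesh components in the construction script from a list of mesh items.
; Each item repeats a set count, advancing a NextPoint cursor by mesh Y length along its yaw and accumulating transform offsets to bend the run.
; Optional join meshes follow each piece or each item.
; Debug arrows and prints remain; the seeded random stream is never sampled.
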(fn `Clear`
  (`|ExecutionSequence`
    (:`then_0`
      (`KismetMathLibrary.SetRandomStreamSeed` (`self.RandomStream`) (`self.Seed`)))
    (:`then_1`
      (`ActorComponent.K2_DestroyComponent` (`self.MainPartMeshList`))
      (`KismetArrayLibrary.Array_Clear` (`self.MainPartMeshList`)))))

(fn `Initialize`
  (set `self.NextPoint` (`KismetMathLibrary.MakeTransform` (0.0 0.0 0.0))))

(fn `RunGeneration`
  (locals (ActualMeshLength :type "Float (double-precision)") (ActualMeshTransform :type "Transform Structure") (ActualMesh :type "StaticMesh Object Reference") (ActualLocalMeshTransform :type "Transform Structure"))
  (bind _actualmeshlength (`local.ActualMeshLength`))
  (bind _actualmeshtransform (`local.ActualMeshTransform`))
  (bind (_joinpartitem_mesh _joinpartitem_itiration _joinpartitem_transform) (break `/Game/SurvivalHorror1/Blueprints/Tools/BP_Mesh_Num_Pos` (`self.JoinPartItem`)))
  (bind (_actuallocalmeshtransform_location _actuallocalmeshtransform_rotation _actuallocalmeshtransform_scale) (`KismetMathLibrary.BreakTransform` (`local.ActualLocalMeshTransform`)))
  (bind _nextpoint (`self.NextPoint`))
  (bind (_joinpartitem_mesh_2 _joinpartitem_itiration_2 _joinpartitem_transform_2) (break `/Game/SurvivalHorror1/Blueprints/Tools/BP_Mesh_Num_Pos` (`self.JoinPartItem`)))
  (bind _returnvalue (`KismetMathLibrary.DegreesToRadians` (.yaw (.rotation _nextpoint))))
  (bind (_returnvalue_roll _returnvalue_pitch _returnvalue_yaw) (`KismetMathLibrary.BreakRotator` (`self.AddRotation` (.rotation _joinpartitem_transform_2) (.rotation (`self.NextPoint`)))))
  (bind (_returnvalue_roll_2 _returnvalue_pitch_2 _returnvalue_yaw_2) (`KismetMathLibrary.BreakRotator` (`self.AddRotation` (.rotation _joinpartitem_transform) (.rotation (`self.NextPoint`)))))
  (bind _returnvalue_2 (+ (.y (.location _nextpoint)) (* _actualmeshlength (`KismetMathLibrary.Sin` _returnvalue))))
  (bind _returnvalue_3 (+ (.x (.location _nextpoint)) (* _actualmeshlength (`KismetMathLibrary.Cos` _returnvalue))))
  (bind _returnvalue_4 (`KismetMathLibrary.MakeTransform` (`KismetMathLibrary.MakeVector` (+ _returnvalue_3 (* (.x (.location _actualmeshtransform)) (.x (.scale _actualmeshtransform)))) (+ _returnvalue_2 (* (.y (.location _actualmeshtransform)) (.y (.scale _actualmeshtransform)))) (+ (.z (.location _nextpoint)) (* (.z (.location _actualmeshtransform)) (.z (.scale _actualmeshtransform))))) (`self.AddRotation` (.rotation (`self.NextPoint`)) (.rotation _actualmeshtransform)) (* (.scale (`self.NextPoint`)) (.scale _actualmeshtransform))))
  (`|ExecutionSequence`
    (:`then_0`
      (`self.Clear`))
    (:`then_1`
      (`self.Initialize`))
    (:`then_2`
      (for _array_element (`self.MainPartItems`)
        (bind (_size_x _size_y) (`KismetMathLibrary.BreakVector` (`self.GetMeshSize` (break `/Game/SurvivalHorror1/Blueprints/Tools/BP_Mesh_Num_Pos` _array_element))))
        (set `local.ActualMeshLength` _size_y)
        (set `local.ActualLocalMeshTransform` (`.Local_Transform_11_478416B442D3EE8DF24E4F877236EEDD` (break `/Game/SurvivalHorror1/Blueprints/Tools/BP_Mesh_Num_Pos` _array_element)))
        (set `local.ActualMeshTransform` (`.Transform_8_639C4F42401392198B5589835F5397C8` (break `/Game/SurvivalHorror1/Blueprints/Tools/BP_Mesh_Num_Pos` _array_element)))
        (set `local.ActualMesh` (break `/Game/SurvivalHorror1/Blueprints/Tools/BP_Mesh_Num_Pos` _array_element))
        (for _ (range (`.Itiration_5_A305B5744295B9884B1F12A7BF5CE1C1` (break `/Game/SurvivalHorror1/Blueprints/Tools/BP_Mesh_Num_Pos` _array_element)))
          (`KismetSystemLibrary.DrawDebugArrow` (`KismetMathLibrary.MakeVector` (.x (.location _nextpoint)) (.y (.location _nextpoint)) 300.0) (`KismetMathLibrary.MakeVector` _returnvalue_3 _returnvalue_2 300.0) (`local.ActualMeshLength`) (struct) 3.0 3.0)
          (bind _returnvalue_5 (`AddComponent|NODE_AddStaticMeshComponent-0`))
          (`KismetArrayLibrary.Array_AddUnique` (`self.MainPartMeshList`) _returnvalue_5)
          (`StaticMeshComponent.SetStaticMesh` _returnvalue_5 (`local.ActualMesh`))
          (`SceneComponent.SetWorldScale3D` _returnvalue_5 (1.0 1.0 1.0))
          (`SceneComponent.K2_AddLocalTransform` _returnvalue_5 (`KismetMathLibrary.MakeTransform` (+ (.location (`KismetMathLibrary.MakeTransform` (`KismetMathLibrary.MakeVector` (- (.x (.location _returnvalue_4)) (`local.ActualMeshLength`)) (.y (.location _returnvalue_4)) (.z (.location _returnvalue_4))) (`KismetMathLibrary.MakeRotator` (.roll (.rotation _returnvalue_4)) (.pitch (.rotation _returnvalue_4)) (+ (.yaw (.rotation _returnvalue_4)) 90.0)) (.scale _returnvalue_4))) _actuallocalmeshtransform_location) (`self.AddRotation` (.rotation (`KismetMathLibrary.MakeTransform` (`KismetMathLibrary.MakeVector` (- (.x (.location _returnvalue_4)) (`local.ActualMeshLength`)) (.y (.location _returnvalue_4)) (.z (.location _returnvalue_4))) (`KismetMathLibrary.MakeRotator` (.roll (.rotation _returnvalue_4)) (.pitch (.rotation _returnvalue_4)) (+ (.yaw (.rotation _returnvalue_4)) 90.0)) (.scale _returnvalue_4))) _actuallocalmeshtransform_rotation) (* (.scale (`KismetMathLibrary.MakeTransform` (`KismetMathLibrary.MakeVector` (- (.x (.location _returnvalue_4)) (`local.ActualMeshLength`)) (.y (.location _returnvalue_4)) (.z (.location _returnvalue_4))) (`KismetMathLibrary.MakeRotator` (.roll (.rotation _returnvalue_4)) (.pitch (.rotation _returnvalue_4)) (+ (.yaw (.rotation _returnvalue_4)) 90.0)) (.scale _returnvalue_4))) _actuallocalmeshtransform_scale)) false true)
          (set `self.NextPoint` _returnvalue_4)
          (if (`self.AddJoin`)
            (bind _returnvalue_6 (`AddComponent|NODE_AddStaticMeshComponent-2`))
            (`KismetArrayLibrary.Array_AddUnique` (`self.MainPartMeshList`) _returnvalue_6)
            (`StaticMeshComponent.SetStaticMesh` _returnvalue_6 _joinpartitem_mesh)
            (`SceneComponent.SetWorldScale3D` _returnvalue_6 (1.0 1.0 1.0))
            (`SceneComponent.K2_SetRelativeTransform` _returnvalue_6 (`KismetMathLibrary.MakeTransform` (`KismetMathLibrary.MakeVector` (- (+ (.x (.location _joinpartitem_transform)) (.x (.location (`self.NextPoint`)))) (`local.ActualMeshLength`)) (+ (.y (.location _joinpartitem_transform)) (.y (.location (`self.NextPoint`)))) (+ (.z (.location _joinpartitem_transform)) (.z (.location (`self.NextPoint`))))) (`KismetMathLibrary.MakeRotator` _returnvalue_roll_2 _returnvalue_pitch_2 (+ _returnvalue_yaw_2 90.0)) (* (.scale _joinpartitem_transform) (.scale (`self.NextPoint`)))) false true)
            (`KismetSystemLibrary.PrintString` (`KismetStringLibrary.Conv_DoubleToString` _returnvalue_yaw_2))))
        (if (`self.ArrayJoin`)
          (bind _returnvalue_7 (`AddComponent|NODE_AddStaticMeshComponent-4`))
          (`KismetArrayLibrary.Array_AddUnique` (`self.MainPartMeshList`) _returnvalue_7)
          (`StaticMeshComponent.SetStaticMesh` _returnvalue_7 _joinpartitem_mesh_2)
          (`SceneComponent.SetWorldScale3D` _returnvalue_7 (1.0 1.0 1.0))
          (`SceneComponent.K2_AddLocalTransform` _returnvalue_7 (`KismetMathLibrary.MakeTransform` (`KismetMathLibrary.MakeVector` (- (+ (.x (.location _joinpartitem_transform_2)) (.x (.location (`self.NextPoint`)))) (`local.ActualMeshLength`)) (+ (.y (.location _joinpartitem_transform_2)) (.y (.location (`self.NextPoint`)))) (+ (.z (.location _joinpartitem_transform_2)) (.z (.location (`self.NextPoint`))))) (`KismetMathLibrary.MakeRotator` _returnvalue_roll _returnvalue_pitch (+ _returnvalue_yaw 90.0)) (* (.scale _joinpartitem_transform_2) (.scale (`self.NextPoint`)))) false true))))))

(fn `UserConstructionScript`
  (`self.RunGeneration`))