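; Inventory component for a survival horror game that holds item slots and toggles the W_Inventory screen.
; BeginPlay fills the slot array with 16 entries, and OpenInventory adds or removes the widget while switching input mode and mouse cursor.
; AddToInventory merges stackable items into a matching unfilled stack, without splitting overflow, or else uses a zero-quantity slot.
; Successful adds refresh any open widget's grid, and the function reports whether the item was added.
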(event `self.ReceiveBeginPlay`
  (for _ (range 16)
    (`KismetArrayLibrary.Array_Add` (`self.Inventory`))))

(event `OpenInventory`
  (bind _returnvalue (`GameplayStatics.GetPlayerController` 0))
  (bind _foundwidgets (`WidgetBlueprintLibrary.GetAllWidgetsOfClass` "/Game/SurvivalHorror1/Blueprints/Inventory_V2/W_Inventory.W_Inventory_C"))
  (bind _output (`|GetArrayItem` _foundwidgets))
  (`/Engine/EditorBlueprintResources/StandardMacros.IsValid` _output
    (:`Is Valid`
      (`Widget.RemoveFromParent` _output)
      (`WidgetBlueprintLibrary.SetInputMode_GameOnly` _returnvalue)
      (set `PlayerController.bShowMouseCursor` false _returnvalue))
    (:`Is Not Valid`
      (bind _returnvalue_2 (`|CreateWidget` "/Game/SurvivalHorror1/Blueprints/Inventory_V2/W_Inventory.W_Inventory_C"))
      (`UserWidget.AddToViewport` _returnvalue_2 0)
      (`WidgetBlueprintLibrary.SetInputMode_GameAndUIEx` _returnvalue null)
      (set `PlayerController.bShowMouseCursor` true _returnvalue))))

(fn `AddToInventory`
  (params (Inventory :type "/Game/SurvivalHorror1/Blueprints/Inventory_V2/ST_Inventory Structure"))
  (returns (ItemAdded :type Boolean) (Item :type "/Game/SurvivalHorror1/Blueprints/Inventory_V2/ST_Inventory Structure"))
  (locals (InventoryREF :type "/Game/SurvivalHorror1/Blueprints/Inventory_V2/ST_Inventory Structure") (IndexREF :type Integer) (Found :type Boolean))
  (bind _inventoryref_name (break `/Game/SurvivalHorror1/Blueprints/Inventory_V2/ST_Inventory` (`local.InventoryREF`)))
  (bind (_output_name _output_description _output_image _output_quantity _output_maxstack _output_stackable _output_value _output_mesh) (break `/Game/SurvivalHorror1/Blueprints/Inventory_V2/ST_Inventory` (`|GetArrayItem` (`self.Inventory`) (`local.IndexREF`))))
  (bind _output_get (set `local.InventoryREF` Inventory))
  (if (`.Stackable_16_6B08D5014EAF0BB330E7D09186A69F10` (break `/Game/SurvivalHorror1/Blueprints/Inventory_V2/ST_Inventory` _output_get))
    (for (_array_element _array_index) (`self.Inventory`)
      (set `local.IndexREF` _array_index)
      (if (and (`KismetTextLibrary.EqualEqual_TextText` (break `/Game/SurvivalHorror1/Blueprints/Inventory_V2/ST_Inventory` _array_element) _inventoryref_name) (< (`.Quantity_8_7115CBFF42C86AAF6C7BDB8EB81F0B48` (break `/Game/SurvivalHorror1/Blueprints/Inventory_V2/ST_Inventory` _array_element)) (`.MaxStack_10_2C084B83491377CB0AA573A707B1D155` (break `/Game/SurvivalHorror1/Blueprints/Inventory_V2/ST_Inventory` _array_element))))
        (set `local.Found` true)
        (break)))
    (if (`local.Found`)
      (`KismetArrayLibrary.Array_Set` (`self.Inventory`) (`local.IndexREF`) (make `/Game/SurvivalHorror1/Blueprints/Inventory_V2/ST_Inventory` _output_name _output_description _output_image (+ _output_quantity (`.Quantity_8_7115CBFF42C86AAF6C7BDB8EB81F0B48` (break `/Game/SurvivalHorror1/Blueprints/Inventory_V2/ST_Inventory` _output_get))) _output_maxstack _output_stackable _output_value _output_mesh))
      (bind _foundwidgets (`WidgetBlueprintLibrary.GetAllWidgetsOfClass` "/Game/SurvivalHorror1/Blueprints/Inventory_V2/W_Inventory.W_Inventory_C"))
      (bind _output (`|GetArrayItem` _foundwidgets))
      (`/Engine/EditorBlueprintResources/StandardMacros.IsValid` _output
        (:`Is Valid`
          (`/Game/SurvivalHorror1/Blueprints/Inventory_V2/W_Inventory.SetGrid` _output))
        (:`Is Not Valid`
          _))
      (return true (`local.InventoryREF`))
      (else
        _)))
  (for (_array_element_2 _array_index_2) (`self.Inventory`)
    (set `local.IndexREF` _array_index_2)
    (if (== (`.Quantity_8_7115CBFF42C86AAF6C7BDB8EB81F0B48` (break `/Game/SurvivalHorror1/Blueprints/Inventory_V2/ST_Inventory` _array_element_2)) 0)
      (set `local.Found` true)
      (break)))
  (if (`local.Found`)
    (`KismetArrayLibrary.Array_Set` (`self.Inventory`) (`local.IndexREF`) (`local.InventoryREF`))
    (bind _foundwidgets_2 (`WidgetBlueprintLibrary.GetAllWidgetsOfClass` "/Game/SurvivalHorror1/Blueprints/Inventory_V2/W_Inventory.W_Inventory_C"))
    (bind _output_2 (`|GetArrayItem` _foundwidgets_2))
    (`/Engine/EditorBlueprintResources/StandardMacros.IsValid` _output_2
      (:`Is Valid`
        (`/Game/SurvivalHorror1/Blueprints/Inventory_V2/W_Inventory.SetGrid` _output_2))
      (:`Is Not Valid`
        _))
    (return true (`local.InventoryREF`))
    (else
      (return false (`local.InventoryREF`)))))