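; BP_Collectable is a pickup actor that adds its item to the player's inventory when interacted with.
; The construction script sets its static mesh from the Inventory item data, so each instance shows the item it holds.
; Interact passes the player to ToInventory, which calls AddToInventory on the MainCharacter's Comp_Inventory.
; On success it refreshes the W_Inventory grid and destroys itself; otherwise it prints that the inventory is full.
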(event `/Game/SurvivalHorror1/Blueprints/Main_Character/BPI_Interact.Interact`
  (params (Player :type "/Game/SurvivalHorror1/Blueprints/Main_Character/BP_MainCharacter Object Reference"))
  (`self.ToInventory` Player))

(event `ToInventory`
  (params (REF :type "/Game/SurvivalHorror1/Blueprints/Main_Character/BP_MainCharacter Object Reference"))
  (bind _asmain_character (cast `MainCharacter` REF))
  (bind _itemadded (`/Game/SurvivalHorror1/Blueprints/Inventory_V2/Comp_Inventory.AddToInventory` (`self.GetComponentByClass` _asmain_character "/Game/SurvivalHorror1/Blueprints/Inventory_V2/Comp_Inventory.Comp_Inventory_C") (`self.Inventory`)))
  (if _itemadded
    (bind _foundwidgets (`WidgetBlueprintLibrary.GetAllWidgetsOfClass` "/Game/SurvivalHorror1/Blueprints/Inventory_V2/W_Inventory.W_Inventory_C"))
    (bind _output (`|GetArrayItem` _foundwidgets))
    (`/Engine/EditorBlueprintResources/StandardMacros.IsValid` _output
      (:`Is Valid`
        (`/Game/SurvivalHorror1/Blueprints/Inventory_V2/W_Inventory.SetGrid` _output))
      (:`Is Not Valid`
        _))
    (`self.K2_DestroyActor`)
    (`KismetSystemLibrary.PrintString` "Item Collected")
    (else
      (`KismetSystemLibrary.PrintString` "Inventory Full"))))

(fn `UserConstructionScript`
  (bind (_inventory_name _inventory_description _inventory_image _inventory_quantity _inventory_maxstack _inventory_stackable _inventory_value _inventory_mesh) (break `/Game/SurvivalHorror1/Blueprints/Inventory_V2/ST_Inventory` (`self.Inventory`)))
  (`StaticMeshComponent.SetStaticMesh` (`self.StaticMesh`) _inventory_mesh))