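; Tutorial trigger volume that teaches the player to interact with items until their first interaction.
; When BP_MainCharacter enters the box, it outlines overlapping BPI_Interact actors with an overlay material and shows an interact message widget.
; On exit, it re-arms and, after a short delay, clears both if the player is still outside.
; PlayerInteract permanently completes the tutorial, removing outlines and closing the widget.
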(event `self.Box.OnComponentBeginOverlap`
  (params (OverlappedComponent :type "PrimitiveComponent Object Reference") (OtherActor :type "Actor Object Reference") (OtherComp :type "PrimitiveComponent Object Reference") (OtherBodyIndex :type Integer) (bFromSweep :type Boolean) (SweepResult :type "HitResult Structure (by ref)"))
  (bind _asbp_main_character (cast `/Game/SurvivalHorror1/Blueprints/Main_Character/BP_MainCharacter` OtherActor))
  (set `self.As BP Main Character` _asbp_main_character)
  (if (and (`KismetSystemLibrary.IsValid` _asbp_main_character) (not (`self.FirstInteractDone`)))
    (`/Engine/EditorBlueprintResources/StandardMacros.DoOnce` false :!label _label
      (:`Completed`
        (`KismetSystemLibrary.PrintString` "Interact tuto show")
        (`KismetArrayLibrary.Array_Clear` (`self.InteractItemsInZone`))
        (for _array_element (`PrimitiveComponent.GetOverlappingActors` (`self.Box`) "/Script/Engine.Actor")
          (if (`KismetSystemLibrary.DoesImplementInterface` _array_element "/Game/SurvivalHorror1/Blueprints/Main_Character/BPI_Interact.BPI_Interact_C")
            (`KismetArrayLibrary.Array_Add` (`self.InteractItemsInZone`) _array_element)))
        (`self.AddOutline`
          (:`Completed`
            (`self.AddWidget`)))))))

(event `self.Box.OnComponentEndOverlap`
  (params (OverlappedComponent :type "PrimitiveComponent Object Reference") (OtherActor :type "Actor Object Reference") (OtherComp :type "PrimitiveComponent Object Reference") (OtherBodyIndex :type Integer))
  (`self.TutoWidget`
    (:`then`
      (if (not (`self.FirstInteractDone`))
        (`|ExecutionSequence`
          (:`then_0`
            (goto _label :!via `Reset`))
          (:`then_1`
            (`KismetSystemLibrary.Delay` 2.0)
            (`/Engine/EditorBlueprintResources/StandardMacros.IsValid` (`|GetArrayItem` (`PrimitiveComponent.GetOverlappingActors` (`self.Box`) "/Game/SurvivalHorror1/Blueprints/Main_Character/BP_MainCharacter.BP_MainCharacter_C"))
              (:`Is Not Valid`
                (`self.RemoveOutline`
                  (:`Completed`
                    (`self.RemoveWidget`)))))))))
    (:`else`)))

(event `/Game/SurvivalHorror1/Blueprints/Tuto/BPI_InteractInput.PlayerInteract`
  (`/Engine/EditorBlueprintResources/StandardMacros.DoOnce` false
    (:`Completed`
      (set `self.FirstInteractDone` true)
      (`KismetSystemLibrary.PrintString` "You interact")
      (`self.RemoveOutline`
        (:`Completed`
          (`self.RemoveWidget`))))))

(fn `UserConstructionScript`)