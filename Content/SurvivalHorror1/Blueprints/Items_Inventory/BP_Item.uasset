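; BP_Item is a world pickup that adds its item info to the interacting player's BP_InventoryManager, then destroys itself, or prints "Inventory full" on failure.
; Its construction script matches the RowName enum to a World_Items data table row by string comparison.
; That row fills ItemInfo, with SpecialValue taken from the actor's own variable, and the item's mesh is applied to the Cube component.
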(event `/Game/SurvivalHorror1/Blueprints/Main_Character/BPI_Interact.Interact`
  (params (Player :type "/Game/SurvivalHorror1/Blueprints/Main_Character/BP_MainCharacter Object Reference"))
  (bind _added (`/Game/SurvivalHorror1/Blueprints/Items_Inventory/BP_InventoryManager.AddToInventory` (`self.GetComponentByClass` Player "/Game/SurvivalHorror1/Blueprints/Items_Inventory/BP_InventoryManager.BP_InventoryManager_C") (`self.Item_info`)))
  (if _added
    (`self.K2_DestroyActor`)
    (else
      (`KismetSystemLibrary.PrintString` "Inventory full"))))

(fn `UserConstructionScript`
  (bind (_item_info_itemname _item_info_itemtype _item_info_description _item_info_itemicon _item_info_itemmesh) (break `/Game/SurvivalHorror1/Blueprints/Items_Inventory/ST_Items` (`self.Item_info`)))
  (bind _out_row_names (`self.Out Row Names`))
  (`|ExecutionSequence`
    (:`then_0`
      (bind _outrownames (`DataTableFunctionLibrary.GetDataTableRowNames` "/Game/SurvivalHorror1/Blueprints/Items_Inventory/World_Items.World_Items"))
      (set `self.Out Row Names` _outrownames)
      (bind _index (`self.GetIndexOfEnum` _out_row_names (`self.Row Name`))
        (:`End`
          (bind _returnvalue (`|GetDataTableRow` "/Game/SurvivalHorror1/Blueprints/Items_Inventory/World_Items.World_Items" (`|GetArrayItem` _out_row_names _index))
            (:`then`
              (bind (_itemname _itemtype _description _itemicon _itemmesh _salable _valuemoney _location) (break `/Game/SurvivalHorror1/Blueprints/Items_Inventory/ST_Items` _returnvalue))
              (set `self.Item_info` (make `/Game/SurvivalHorror1/Blueprints/Items_Inventory/ST_Items` _itemname _itemtype _description _itemicon _itemmesh _salable _valuemoney _location (`self.SpecialValue`))))))))
    (:`then_1`
      (`StaticMeshComponent.SetStaticMesh` (`self.Cube`) _item_info_itemmesh))))