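; BP_InventoryManager runs the player's inventory and five-slot hotbar, toggling the W_Inv widget and equipping hotbar items by input.
; Added items fill the hotbar before the inventory, save to SG_Inventory and refresh the grid.
; Equipping resolves World_Items row names to an enum, toggling lantern or gun with animation and a cooldown flag.
; The branch for dequipping a different held item is unconnected.
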(event `self.ReceiveBeginPlay`
  (`self.LoadInventory`)
  (bind _returnvalue (`|CreateWidget` "/Game/SurvivalHorror1/Blueprints/Items_Inventory/W_Inv.W_Inv_C"))
  (set `self.InventoryWidget` _returnvalue)
  (`UserWidget.AddToViewport` _returnvalue 0)
  (`self.CloseInventory`)
  (bind _asbp_main_character (cast `/Game/SurvivalHorror1/Blueprints/Main_Character/BP_MainCharacter` (`GameplayStatics.GetPlayerCharacter` 0)))
  (set `self.MainCharacterREF` _asbp_main_character))

(event `InputAction|Inventory`
  (params (Key :type "Key Structure"))
  (:`Pressed`
    (if (`self.InventoryOpen?`)
      (`self.CloseInventory`)
      (set `self.InventoryOpen?` false)
      (else
        (`self.OpenInventory`)
        (set `self.InventoryOpen?` true)))))

(event `InputAction|Item1`
  (params (Key :type "Key Structure"))
  (:`Pressed`
    (`self.EquipItem` (`|GetArrayItem` (`self.Hotbar`)))))

(event `InputAction|Item2`
  (params (Key :type "Key Structure"))
  (:`Pressed`
    (`self.EquipItem` (`|GetArrayItem` (`self.Hotbar`) 1))))

(event `InputAction|Item3`
  (params (Key :type "Key Structure"))
  (:`Pressed`
    (`self.EquipItem` (`|GetArrayItem` (`self.Hotbar`) 2))))

(event `InputAction|Item4`
  (params (Key :type "Key Structure"))
  (:`Pressed`
    (`self.EquipItem` (`|GetArrayItem` (`self.Hotbar`) 3))))

(event `InputAction|Item5`
  (params (Key :type "Key Structure"))
  (:`Pressed`
    (`self.EquipItem` (`|GetArrayItem` (`self.Hotbar`) 4))))

(event `EquipLantern`
  (bind _maincharacterref (`self.MainCharacterREF`))
  (if (`self.CanTakeItemOut?`)
    (set `self.CanTakeItemOut?` false)
    (set `/Game/SurvivalHorror1/Blueprints/Main_Character/BP_Anim_MainCharacter.LeftArmHolding` 2 (`/Game/SurvivalHorror1/Blueprints/Main_Character/BP_MainCharacter.Anim Main Character REF` _maincharacterref))
    (`Character.PlayAnimMontage` _maincharacterref "/Game/SurvivalHorror1/Art/MainCharacter/Lantern_idle_Anim_Montage.Lantern_idle_Anim_Montage" 1.0 "None")
    (`GameplayStatics.PlaySound2D` "/Game/SurvivalHorror1/Sound/Effects/allumage_lampe.allumage_lampe" 1.0 1.0 0.0 null null)
    (`SceneComponent.SetHiddenInGame` (`/Game/SurvivalHorror1/Blueprints/Main_Character/BP_MainCharacter.lantern` _maincharacterref) false true)
    (`LightComponent.SetIntensity` (`/Game/SurvivalHorror1/Blueprints/Main_Character/BP_MainCharacter.Lamp` _maincharacterref) 30.0)
    (`KismetSystemLibrary.Delay` 0.5)
    (set `/Game/SurvivalHorror1/Blueprints/Main_Character/BP_Anim_MainCharacter.LeftArmHolding` 1 (`/Game/SurvivalHorror1/Blueprints/Main_Character/BP_MainCharacter.Anim Main Character REF` (`self.MainCharacterREF`)))
    (set `self.CanTakeItemOut?` true)
    (bind _returnvalue (`GameplayStatics.SpawnSound2D` "/Game/SurvivalHorror1/Sound/Effects/lampe_loupe.lampe_loupe" 1.0 1.0 0.0 null))
    (set `self.LanternSoundLoop` _returnvalue)
    (else
      (set `self.CanTakeItemOut?` true))))

(event `DequipLantern`
  (bind _maincharacterref (`self.MainCharacterREF`))
  (bind _lanternsoundloop (`self.LanternSoundLoop`))
  (if (`self.CanTakeItemOut?`)
    (set `self.CanTakeItemOut?` false)
    (set `/Game/SurvivalHorror1/Blueprints/Main_Character/BP_Anim_MainCharacter.LeftArmHolding` 3 (`/Game/SurvivalHorror1/Blueprints/Main_Character/BP_MainCharacter.Anim Main Character REF` _maincharacterref))
    (`LightComponent.SetIntensity` (`/Game/SurvivalHorror1/Blueprints/Main_Character/BP_MainCharacter.Lamp` _maincharacterref) 0.0)
    (`Character.StopAnimMontage` _maincharacterref "/Game/SurvivalHorror1/Art/MainCharacter/Lantern_idle_Anim_Montage.Lantern_idle_Anim_Montage")
    (`SceneComponent.SetHiddenInGame` (`/Game/SurvivalHorror1/Blueprints/Main_Character/BP_MainCharacter.lantern` _maincharacterref) true true)
    (set `/Game/SurvivalHorror1/Blueprints/Main_Character/BP_Anim_MainCharacter.LeftArmHolding` 0 (`/Game/SurvivalHorror1/Blueprints/Main_Character/BP_MainCharacter.Anim Main Character REF` (`self.MainCharacterREF`)))
    (`/Engine/EditorBlueprintResources/StandardMacros.IsValid` _lanternsoundloop
      (:`Is Valid`
        (`AudioComponent.FadeOut` _lanternsoundloop 0.5 0.0 "Linear"))
      (:`Is Not Valid`
        _))
    (`KismetSystemLibrary.RetriggerableDelay` 0.5)
    (set `self.CanTakeItemOut?` true)
    (else
      (set `self.CanTakeItemOut?` true))))

(event `EquipGun`
  (bind _maincharacterref (`self.MainCharacterREF`))
  (if (`self.CanTakeItemOut?`)
    (set `self.CanTakeItemOut?` false)
    (set `/Game/SurvivalHorror1/Blueprints/Main_Character/BP_Anim_MainCharacter.LeftArmHolding` 2 (`/Game/SurvivalHorror1/Blueprints/Main_Character/BP_MainCharacter.Anim Main Character REF` _maincharacterref))
    (`Character.PlayAnimMontage` _maincharacterref "/Game/SurvivalHorror1/Art/MainCharacter/Lantern_idle_Anim_Montage.Lantern_idle_Anim_Montage" 1.0 "None")
    (`SceneComponent.SetHiddenInGame` (`/Game/SurvivalHorror1/Blueprints/Main_Character/BP_MainCharacter.Gun` _maincharacterref) false true)
    (`KismetSystemLibrary.Delay` 0.5)
    (set `/Game/SurvivalHorror1/Blueprints/Main_Character/BP_MainCharacter.GunUp?` true (`self.MainCharacterREF`))
    (bind _returnvalue (`|CreateWidget` "/Game/SurvivalHorror1/Blueprints/Menu/pointer.pointer_C"))
    (set `self.Pointer` _returnvalue)
    (`UserWidget.AddToViewport` _returnvalue 0)
    (set `/Game/SurvivalHorror1/Blueprints/Main_Character/BP_Anim_MainCharacter.LeftArmHolding` 1 (`/Game/SurvivalHorror1/Blueprints/Main_Character/BP_MainCharacter.Anim Main Character REF` (`self.MainCharacterREF`)))
    (set `self.CanTakeItemOut?` true)
    (else
      (set `self.CanTakeItemOut?` true))))

(event `DequipGun`
  (bind _pointer (`self.Pointer`))
  (bind _maincharacterref (`self.MainCharacterREF`))
  (if (`self.CanTakeItemOut?`)
    (set `self.CanTakeItemOut?` false)
    (set `/Game/SurvivalHorror1/Blueprints/Main_Character/BP_MainCharacter.GunUp?` false (`self.MainCharacterREF`))
    (`/Engine/EditorBlueprintResources/StandardMacros.IsValid` _pointer
      (:`Is Valid`
        (`Widget.RemoveFromParent` _pointer))
      (:`Is Not Valid`
        _))
    (set `/Game/SurvivalHorror1/Blueprints/Main_Character/BP_Anim_MainCharacter.LeftArmHolding` 3 (`/Game/SurvivalHorror1/Blueprints/Main_Character/BP_MainCharacter.Anim Main Character REF` _maincharacterref))
    (`KismetSystemLibrary.RetriggerableDelay` 0.5)
    (`Character.StopAnimMontage` _maincharacterref "/Game/SurvivalHorror1/Art/MainCharacter/Lantern_idle_Anim_Montage.Lantern_idle_Anim_Montage")
    (`SceneComponent.SetHiddenInGame` (`/Game/SurvivalHorror1/Blueprints/Main_Character/BP_MainCharacter.Gun` _maincharacterref) true true)
    (set `/Game/SurvivalHorror1/Blueprints/Main_Character/BP_Anim_MainCharacter.LeftArmHolding` 0 (`/Game/SurvivalHorror1/Blueprints/Main_Character/BP_MainCharacter.Anim Main Character REF` (`self.MainCharacterREF`)))
    (set `self.CanTakeItemOut?` true)
    (else
      (set `self.CanTakeItemOut?` true))))

(fn `AddToInventory`
  (params (Item :type "/Game/SurvivalHorror1/Blueprints/Items_Inventory/ST_Items Structure"))
  (returns (Added :type Boolean))
  (locals (ItemToAdd :type "/Game/SurvivalHorror1/Blueprints/Items_Inventory/ST_Items Structure") (SlotIn :type Integer))
  (set `local.ItemToAdd` Item)
  (bind (_slotfind _idslot) (`self.Get Empty Slot` (`self.Hotbar`)))
  (set `local.SlotIn` _idslot)
  (if _slotfind
    (set `local.ItemToAdd` (`self.SetItemLocation` (`local.ItemToAdd`)))
    (`KismetArrayLibrary.Array_Set` (`self.Hotbar`) (`local.SlotIn`) (`local.ItemToAdd`))
    (`self.SaveInventory`)
    (`self.SetGrid`
      (:`Out`
        (return true)))
    (else
      (bind (_slotfind_2 _idslot_2) (`self.Get Empty Slot` (`self.Inventory`)))
      (set `local.SlotIn` _idslot_2)
      (if _slotfind_2
        (set `local.ItemToAdd` (`self.SetItemLocation` (`local.ItemToAdd`) "NewEnumerator1"))
        (`KismetArrayLibrary.Array_Set` (`self.Inventory`) (`local.SlotIn`) (`local.ItemToAdd`))
        (`self.SaveInventory`)
        (`self.SetGrid`
          (:`Out`
            (return true)))
        (else
          (return false))))))

(fn `CloseInventory`
  (bind _returnvalue (`GameplayStatics.GetPlayerController` 0))
  (`Widget.SetVisibility` (`self.InventoryWidget`) "Hidden")
  (`WidgetBlueprintLibrary.SetInputMode_GameOnly` _returnvalue)
  (set `PlayerController.bShowMouseCursor` false _returnvalue))

(fn `EquipItem`
  (params (ItemToEquip :type "/Game/SurvivalHorror1/Blueprints/Items_Inventory/ST_Items Structure"))
  (locals (ItemIn :type "/Game/SurvivalHorror1/Blueprints/Items_Inventory/ST_Items Structure"))
  (bind _output_get (set `local.ItemIn` ItemToEquip))
  (switch `/Game/SurvivalHorror1/Blueprints/Items_Inventory/Item_Types` (`.ItemType_10_9A94A55D4971757E24B76EB343586F45` (break `/Game/SurvivalHorror1/Blueprints/Items_Inventory/ST_Items` _output_get))
    (:`NewEnumerator1`
      (set `self.ItemEquiped` (`local.ItemIn`)))
    (:`NewEnumerator4`
      (bind _itemrowname (`self.getItemRowName` (break `/Game/SurvivalHorror1/Blueprints/Items_Inventory/ST_Items` _output_get))
        (:`execout`
          (bind (_finded_1 _itemenum1) (`self.Get Item Enum` _itemrowname))
          (if _finded_1
            (switch `/Game/SurvivalHorror1/Blueprints/Items_Inventory/All_Items` _itemenum1
              (:`NewEnumerator5`
                (`self.CheckEquipement` (`local.ItemIn`)
                  (:`dequip`
                    (`self.DequipLantern`)
                    (set `self.AbilityEquiped` (struct)))
                  (:`equip`
                    (`self.EquipLantern`)
                    (set `self.AbilityEquiped` (`local.ItemIn`)))))
              (:`NewEnumerator6`
                (`self.CheckEquipement` (`local.ItemIn`)
                  (:`dequip`
                    (`self.DequipGun`)
                    (set `self.AbilityEquiped` (struct)))
                  (:`equip`
                    (`self.EquipGun`)
                    (set `self.AbilityEquiped` (`local.ItemIn`))))))))))))

(fn `Get Empty Slot`
  (params (ItemsStorage :type "Array of /Game/SurvivalHorror1/Blueprints/Items_Inventory/ST_Items Structure"))
  (returns (SlotFind :type Boolean) (IdSlot :type Integer))
  (locals (Index :type Integer) (Finded :type Boolean))
  (for (_array_element _array_index) ItemsStorage
    (set `local.Index` _array_index)
    (bind _output_get (set `local.Finded` (== (break `/Game/SurvivalHorror1/Blueprints/Items_Inventory/ST_Items` _array_element) "None")))
    (if _output_get
      (break)))
  (return (`local.Finded`) (`local.Index`)))

(fn `Get Item Enum`
  (params (ItameRowName :type Name))
  (returns (`Finded?1` :type Boolean) (ItemEnum1 :type "/Game/SurvivalHorror1/Blueprints/Items_Inventory/All_Items Enum"))
  (locals (`Finded?` :type Boolean) (ItemEnum :type "/Game/SurvivalHorror1/Blueprints/Items_Inventory/All_Items Enum"))
  (bind _enumvalue (foreach `/Game/SurvivalHorror1/Blueprints/Items_Inventory/All_Items` false)
    (:`LoopBody`
      (if (== ItameRowName (`|GetEnumeratorNameAsString` _enumvalue))
        (set `local.Finded?` true)
        (set `local.ItemEnum` _enumvalue)))
    (:`then`
      (return (`local.Finded?`) (`local.ItemEnum`)))))

(fn `LoadInventory`
  (bind _returnvalue (`GameplayStatics.DoesSaveGameExist` (`self.Slot Name`)))
  (if _returnvalue
    (bind _returnvalue_2 (`GameplayStatics.LoadGameFromSlot` (`self.Slot Name`)))
    (bind _assg_inventory (cast `/Game/SurvivalHorror1/Blueprints/Items_Inventory/SG_Inventory` _returnvalue_2))
    (set `self.Inventory` (`/Game/SurvivalHorror1/Blueprints/Items_Inventory/SG_Inventory.Inventory` _assg_inventory))
    (set `self.Hotbar` (`/Game/SurvivalHorror1/Blueprints/Items_Inventory/SG_Inventory.Hotbar` _assg_inventory))
    (else
      (for _ (range 15)
        (`KismetArrayLibrary.Array_Add` (`self.Inventory`) (make `/Game/SurvivalHorror1/Blueprints/Items_Inventory/ST_Items` "None" "NewEnumerator5" "" null null false 0 "NewEnumerator1")))
      (for _ (range 5)
        (`KismetArrayLibrary.Array_Add` (`self.Hotbar`) (make `/Game/SurvivalHorror1/Blueprints/Items_Inventory/ST_Items` "None" "NewEnumerator5" "" null null false 0 "NewEnumerator0"))))))

(fn `OpenInventory`
  (bind _returnvalue (`GameplayStatics.GetPlayerController` 0))
  (bind _inventorywidget (`self.InventoryWidget`))
  (`Widget.SetVisibility` _inventorywidget "Visible")
  (`WidgetBlueprintLibrary.SetInputMode_GameAndUIEx` _returnvalue _inventorywidget "DoNotLock" false)
  (set `PlayerController.bShowMouseCursor` true _returnvalue))

(fn `RemoveFromInventory`
  (params (Item :type "/Game/SurvivalHorror1/Blueprints/Items_Inventory/ST_Items Structure"))
  (returns (`Removed?` :type Boolean))
  (bind _hotbar (`self.Hotbar`))
  (bind _inventory (`self.Inventory`))
  (switch `/Game/SurvivalHorror1/Blueprints/Items_Inventory/Item_Location` Item_Location_43_D71AD795425EB4125E532DBB62FC5B1B
    (:`NewEnumerator0`
      (for (_array_element _array_index) _hotbar
        (if (== (break `/Game/SurvivalHorror1/Blueprints/Items_Inventory/ST_Items` _array_element) Item_ItemName_13_3536A9694BC1016CF006F3BFC8AE3C0B)
          (`|ExecutionSequence`
            (:`then_0`
              (break))
            (:`then_1`
              (`KismetArrayLibrary.Array_Set` _hotbar _array_index)
              (return true)))))
      (return false))
    (:`NewEnumerator1`
      (for (_array_element_2 _array_index_2) _inventory
        (if (== (break `/Game/SurvivalHorror1/Blueprints/Items_Inventory/ST_Items` _array_element_2) Item_ItemName_13_3536A9694BC1016CF006F3BFC8AE3C0B)
          (`|ExecutionSequence`
            (:`then_0`
              (break))
            (:`then_1`
              (`KismetArrayLibrary.Array_Set` _inventory _array_index_2)
              (return true)))))
      (return false))))

(fn `SaveInventory`
  (bind _returnvalue (`GameplayStatics.DoesSaveGameExist` (`self.Slot Name`)))
  (if _returnvalue
    (bind _returnvalue_2 (`GameplayStatics.LoadGameFromSlot` (`self.Slot Name`)))
    (bind _output_get (set `self.SGRef` _returnvalue_2))
    (else
      (bind _returnvalue_3 (`GameplayStatics.CreateSaveGameObject` "/Game/SurvivalHorror1/Blueprints/Items_Inventory/SG_Inventory.SG_Inventory_C"))
      (set `self.SGRef` _returnvalue_3)))
  (bind _assg_inventory (cast `/Game/SurvivalHorror1/Blueprints/Items_Inventory/SG_Inventory` _output_get))
  (set `/Game/SurvivalHorror1/Blueprints/Items_Inventory/SG_Inventory.Inventory` (`self.Inventory`) _assg_inventory)
  (set `/Game/SurvivalHorror1/Blueprints/Items_Inventory/SG_Inventory.Hotbar` (`self.Hotbar`) _assg_inventory)
  (`GameplayStatics.SaveGameToSlot` (`self.SGRef`) (`self.Slot Name`))
  (`KismetSystemLibrary.PrintString` "Inventory and Hotbar Saved"))