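; GameplayAbilityPickUp is an interactable pickup that grants a gameplay ability to a player.
; Its construction script applies the configured Niagara system to the pickup's display effect.
; On Interact, if the player implements UsesAbilities, it spawns an ability actor at the collision sphere, initialized with the pickup's settings, and passes it and itself via PickupAbilityMessage.
; The ability type selects the spawned class, with only Fire implemented.
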(event `/Game/SurvivalHorror1/Blueprints/Main_Character/BPI_Interact.Interact`
  (params (Player :type "/Game/SurvivalHorror1/Blueprints/Main_Character/BP_MainCharacter Object Reference"))
  (if (`KismetSystemLibrary.DoesImplementInterface` Player "/Game/SurvivalHorror1/Blueprints/GameplayAbilityPickUp/UsesAbilities.UsesAbilities_C")
    (bind _returnvalue (`self.SpawnGameplayAbility`))
    (message `/Game/SurvivalHorror1/Blueprints/GameplayAbilityPickUp/UsesAbilities.PickupAbility` Player _returnvalue self)))

(fn `SpawnGameplayAbility`
  (returns (ReturnValue :type "/Game/SurvivalHorror1/Blueprints/GameplayAbilities/GameplayAbilityFire Object Reference"))
  (switch `/Game/SurvivalHorror1/Blueprints/GameplayAbilities/GameplayAbilityType` (`self.AbilityTye`)
    (:`NewEnumerator0`
      (bind _returnvalue (`|SpawnActorFromClass` "/Game/SurvivalHorror1/Blueprints/GameplayAbilities/GameplayAbilityFire.GameplayAbilityFire_C" (`SceneComponent.K2_GetComponentToWorld` (`self.PickUpCollisionSphere`)) "Undefined" "OverrideRootScale" null (`self.Intensity`) (`self.AbilityTye`) (`self.How Ggameplay Ablity Is Used`) (`self.AbilityIcon`) null))
      (return _returnvalue))))

(fn `UserConstructionScript`
  (`NiagaraComponent.SetAsset` (`self.PickUpNiagraSystemEffect`) (`self.NiagraSystemDisplay`) true))