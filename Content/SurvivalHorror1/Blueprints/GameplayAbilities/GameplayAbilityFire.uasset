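; Fire gameplay ability for the main character that raises and lowers a lit lantern from the hotbar, implementing only the Display Only usage mode.
; Activation and deactivation drive the left-arm AnimBP state, idle montage, lantern visibility and lamp intensity across timed delays.
; A flag blocks toggling during transitions.
; Deactivation resets the hotbar, clears the character's active ability and fires any pending hotbar key press.
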(event `self.ReceiveBeginPlay`
  (`self.MainCharacterREFDEF`)
  (`self.ABP_MainCharacterREF`))

(event `ActivateFireAbility`
  (bind _maincharactereref (`self.MainCharactereREF`))
  (bind _maincharactereref_2 (`self.MainCharactereREF`))
  (bind _maincharactereref_3 (`self.MainCharactereREF`))
  (switch `/Game/SurvivalHorror1/Blueprints/GameplayAbilities/HowGgameplayAblityIsUsed` (`self.HowGameplayAblityIsUsed`)
    (:`NewEnumerator0`
      (set `self.AbleToBeActivatedOrDeactivated` false)
      (set `/Game/SurvivalHorror1/Art/MainCharacter/Animation/Arm_AnimBP.LeftArmHoldingUp` 2 (`/Game/SurvivalHorror1/Blueprints/Main_Character/BP_MainCharacter.Anim BPREF` _maincharactereref_2))
      (`Character.PlayAnimMontage` _maincharactereref_3 "/Game/SurvivalHorror1/Art/MainCharacter/Lantern_idle_Anim_Montage.Lantern_idle_Anim_Montage" 1.0 "None")
      (`SceneComponent.SetHiddenInGame` (`/Game/SurvivalHorror1/Blueprints/Main_Character/BP_MainCharacter.lantern` _maincharactereref_3) false true)
      (`LightComponent.SetIntensity` (`/Game/SurvivalHorror1/Blueprints/Main_Character/BP_MainCharacter.Lamp` _maincharactereref_2) 500.0)
      (`KismetSystemLibrary.Delay` 2.0)
      (set `/Game/SurvivalHorror1/Art/MainCharacter/Animation/Arm_AnimBP.LeftArmHoldingUp` 1 (`/Game/SurvivalHorror1/Blueprints/Main_Character/BP_MainCharacter.Anim BPREF` (`self.MainCharactereREF`)))
      (set `self.AbleToBeActivatedOrDeactivated` true)
      (`/Game/SurvivalHorror1/Blueprints/Main_Character/BP_MainCharacter.ActivateHotbarButton` _maincharactereref (`/Game/SurvivalHorror1/Blueprints/Main_Character/BP_MainCharacter.ActiveHotbarSlot` _maincharactereref)))))

(event `DeactivateFireAbility`
  (bind _maincharactereref (`self.MainCharactereREF`))
  (bind _maincharactereref_2 (`self.MainCharactereREF`))
  (bind _activatedgameplayability (`/Game/SurvivalHorror1/Blueprints/Main_Character/BP_MainCharacter.ActivatedGameplayAbility` _maincharactereref_2))
  (set `self.AbleToBeActivatedOrDeactivated` false)
  (switch `/Game/SurvivalHorror1/Blueprints/GameplayAbilities/HowGgameplayAblityIsUsed` (`self.HowGameplayAblityIsUsed`)
    (:`NewEnumerator0`
      (set `/Game/SurvivalHorror1/Art/MainCharacter/Animation/Arm_AnimBP.LeftArmHoldingUp` 3 (`/Game/SurvivalHorror1/Blueprints/Main_Character/BP_MainCharacter.Anim BPREF` _maincharactereref))
      (`KismetSystemLibrary.RetriggerableDelay` 2.0)
      (`LightComponent.SetIntensity` (`/Game/SurvivalHorror1/Blueprints/Main_Character/BP_MainCharacter.Lamp` _maincharactereref) 0.0)
      (`Character.StopAnimMontage` (`self.MainCharactereREF`) "/Game/SurvivalHorror1/Art/MainCharacter/Lantern_idle_Anim_Montage.Lantern_idle_Anim_Montage")
      (`SceneComponent.SetHiddenInGame` (`/Game/SurvivalHorror1/Blueprints/Main_Character/BP_MainCharacter.lantern` _maincharactereref) true true)
      (set `/Game/SurvivalHorror1/Art/MainCharacter/Animation/Arm_AnimBP.LeftArmHoldingUp` 0 (`/Game/SurvivalHorror1/Blueprints/Main_Character/BP_MainCharacter.Anim BPREF` (`self.MainCharactereREF`)))
      (`/Game/SurvivalHorror1/Blueprints/Main_Character/BP_MainCharacter.RestoreHotbarButtonToDefault` _maincharactereref_2)
      (set `/Game/SurvivalHorror1/Blueprints/Main_Character/BP_MainCharacter.HotbarSlotActive?` false _maincharactereref_2)
      (`/Engine/EditorBlueprintResources/StandardMacros.IsValid` _activatedgameplayability
        (:`Is Valid`
          (set `/Game/SurvivalHorror1/Blueprints/GameplayAbilities/GameplayAbility.AbleToBeActivatedOrDeactivated` true _activatedgameplayability)
          (set `/Game/SurvivalHorror1/Blueprints/Main_Character/BP_MainCharacter.ActivatedGameplayAbility` null _maincharactereref_2)
          (if (`/Game/SurvivalHorror1/Blueprints/Main_Character/BP_MainCharacter.KeyboardButtonPerdingActivation?` _maincharactereref_2)
            (`/Game/SurvivalHorror1/Blueprints/Main_Character/BP_MainCharacter.OverallHotbarAbility` _maincharactereref_2 (`/Game/SurvivalHorror1/Blueprints/Main_Character/BP_MainCharacter.KeyboardButtonPendingActivation` _maincharactereref_2))))))))

(fn `UserConstructionScript`
  (`parent.UserConstructionScript`))