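; GameplayAbility is a base Blueprint for player abilities, with shared activate and deactivate events.
; Both events check an AbleToBeActivatedOrDeactivated flag, switch on AbilityType, and cast self to the child class; only Fire is handled, through GameplayAbilityFire.
; BeginPlay caches the BP_MainCharacter reference from the player character, while the animation Blueprint reference function it also calls is empty.
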(event `self.ReceiveBeginPlay`
  (`self.MainCharacterREFDEF`)
  (`self.ABP_MainCharacterREF`))

(event `ActivateAbility`
  (if (`self.AbleToBeActivatedOrDeactivated`)
    (switch `/Game/SurvivalHorror1/Blueprints/GameplayAbilities/GameplayAbilityType` (`self.AbilityType`)
      (:`NewEnumerator0`
        (bind _asgameplay_ability_fire (cast `/Game/SurvivalHorror1/Blueprints/GameplayAbilities/GameplayAbilityFire` self))
        (`/Game/SurvivalHorror1/Blueprints/GameplayAbilities/GameplayAbilityFire.ActivateFireAbility` _asgameplay_ability_fire)))))

(event `DeactivateAbility`
  (if (`self.AbleToBeActivatedOrDeactivated`)
    (switch `/Game/SurvivalHorror1/Blueprints/GameplayAbilities/GameplayAbilityType` (`self.AbilityType`)
      (:`NewEnumerator0`
        (bind _asgameplay_ability_fire (cast `/Game/SurvivalHorror1/Blueprints/GameplayAbilities/GameplayAbilityFire` self))
        (`/Game/SurvivalHorror1/Blueprints/GameplayAbilities/GameplayAbilityFire.DeactivateFireAbility` _asgameplay_ability_fire)))))

(fn `ABP_MainCharacterREF`)

(fn `MainCharacterREFDEF`
  (bind _asbp_main_character (cast `/Game/SurvivalHorror1/Blueprints/Main_Character/BP_MainCharacter` (`GameplayStatics.GetPlayerCharacter` 0)))
  (set `self.MainCharactereREF` _asbp_main_character))

(fn `UserConstructionScript`)