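; Actor component that gives its owner's skeletal mesh partial physical animation, using a profile named HitReaction.
; BeginPlay adds a PhysicalAnimationComponent to the owner and binds it to the first SkeletalMeshComponent found.
; TogglePhysicalAnimation simulates all bodies below Root, applies the profile and sets a half physics blend weight.
; Despite its name, it only enables the effect; the BP_MainCharacter cast and strength multiplier nodes are unconnected.
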(event `self.ReceiveBeginPlay`
  (bind _returnvalue (`self.GetOwner`))
  (bind _returnvalue_2 (`Actor.GetComponentByClass` _returnvalue "/Script/Engine.SkeletalMeshComponent"))
  (bind _returnvalue_3 (`|AddComponentByClass` _returnvalue "/Script/Engine.PhysicalAnimationComponent"))
  (bind _output_get (set `self.PhysicalAnimationComponent` _returnvalue_3))
  (`PhysicalAnimationComponent.SetSkeletalMeshComponent` _output_get _returnvalue_2)
  (set `self.SkeletalMeshComponent` _returnvalue_2))

(event `TogglePhysicalAnimation`
  (bind _skeletalmeshcomponent (`self.SkeletalMeshComponent`))
  (`SkeletalMeshComponent.SetAllBodiesBelowSimulatePhysics` _skeletalmeshcomponent "Root" true false)
  (`PhysicalAnimationComponent.ApplyPhysicalAnimationProfileBelow` (`self.PhysicalAnimationComponent`) "Root" "HitReaction" false false)
  (`SkeletalMeshComponent.SetAllBodiesBelowPhysicsBlendWeight` _skeletalmeshcomponent "Root" 0.5 false false))