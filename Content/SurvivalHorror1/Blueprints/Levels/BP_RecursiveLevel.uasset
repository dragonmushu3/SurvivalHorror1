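; BP_RecursiveLevel is a level streaming actor that manages a level instance and a list of nested recursive levels.
; Load streams in its Level by soft reference, while the construction script also calls level-instance loading without passing Level.
; Unload loops through the list, unloading each entry, setting the streaming level's unload-and-removal request to false and calling DestroyActor.
; The construction script's cascade that would load the listed entries is disconnected.
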(fn `Load`
  (`LevelStreamingDynamic.LoadLevelInstanceBySoftObjectPtr` :`self` (`self.LevelStreamingDynRef`) :`Level` (`self.Level`) :`OptionalLevelStreamingClass` null))

(fn `Unload`
  (for _array_element (`self.RecursiveLevelList`)
    (`self.Unload` _array_element)
    (`LevelStreaming.SetIsRequestingUnloadAndRemoval` (`self.LevelStreamingDynRef`) false)
    (`self.K2_DestroyActor`)))

(fn `UserConstructionScript`
  (`LevelStreamingDynamic.LoadLevelInstanceBySoftObjectPtr` :`self` (`self.LevelStreamingDynRef`) :`OptionalLevelStreamingClass` null))