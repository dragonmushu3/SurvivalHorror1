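; BP_WineFuser is the input side of a wine fusing puzzle, accepting a full wine bottle, a Barron bottle and grass from the player's equipped item.
; Interact runs only while BP_WineFuserOut is not interactable, resolving the item name through World_Items row names to an item enum.
; Each new ingredient fills its mesh slot and leaves the inventory.
; After a short delay, the first BP_WineFuserOut found receives this actor via SendWineInfoMessage.
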(event `/Game/SurvivalHorror1/Blueprints/Main_Character/BPI_Interact.Interact`
  (params (Player :type "/Game/SurvivalHorror1/Blueprints/Main_Character/BP_MainCharacter Object Reference"))
  (bind (_interactitem_itemname _interactitem_itemtype _interactitem_description _interactitem_itemicon _interactitem_itemmesh) (break `/Game/SurvivalHorror1/Blueprints/Items_Inventory/ST_Items` (`self.InteractItem`)))
  (bind _bp_inventorymanager (`/Game/SurvivalHorror1/Blueprints/Main_Character/BP_MainCharacter.BP_InventoryManager` (`self.Player`)))
  (bind _output_get (set `self.Player` Player))
  (set `self.InteractItem` (`/Game/SurvivalHorror1/Blueprints/Items_Inventory/BP_InventoryManager.ItemEquiped` (`/Game/SurvivalHorror1/Blueprints/Main_Character/BP_MainCharacter.BP_InventoryManager` _output_get)))
  (bind _outactors (`GameplayStatics.GetAllActorsOfClass` "/Game/SurvivalHorror1/Blueprints/Furniture/BP_WineFuserOut.BP_WineFuserOut_C"))
  (if (`/Game/SurvivalHorror1/Blueprints/Furniture/BP_WineFuserOut.Interactable?` (`|GetArrayItem` _outactors))
    _
    (elif (`self.Interactable?`)
      (set `self.Interactable?` false)
      (bind _itemrowname (`self.getItemRowName` _interactitem_itemname)
        (:`execout`
          (bind (_finded_1 _itemenum1) (`self.Get Item Enum` _itemrowname))
          (if _finded_1
            (switch `/Game/SurvivalHorror1/Blueprints/Items_Inventory/All_Items` _itemenum1
              (:`NewEnumerator1`
                (if (not (`self.WineIn?`))
                  (`StaticMeshComponent.SetStaticMesh` (`self.Slot2`) _interactitem_itemmesh)
                  (set `self.WineIn?` true)
                  (`/Game/SurvivalHorror1/Blueprints/Items_Inventory/BP_InventoryManager.RemoveFromInventory` _bp_inventorymanager (`self.InteractItem`) :!label _label)
                  (set `/Game/SurvivalHorror1/Blueprints/Items_Inventory/BP_InventoryManager.ItemEquiped` (struct) _bp_inventorymanager)
                  (`KismetSystemLibrary.RetriggerableDelay` 2.0)
                  (bind _outactors_2 (`GameplayStatics.GetAllActorsOfClass` "/Game/SurvivalHorror1/Blueprints/Furniture/BP_WineFuserOut.BP_WineFuserOut_C"))
                  (message `/Game/SurvivalHorror1/Blueprints/Furniture/BPI_WineCom.SendWineInfo` (`|GetArrayItem` _outactors_2) (`self.Player`) self)
                  (set `self.Interactable?` true)
                  (else
                    (set `self.Interactable?` true :!label _label_2))))
              (:`NewEnumerator2`
                (if (not (`self.BottleIn?`))
                  (`StaticMeshComponent.SetStaticMesh` (`self.Slot1`) _interactitem_itemmesh)
                  (set `self.BottleIn?` true)
                  (goto _label)
                  (else
                    (goto _label_2))))
              (:`NewEnumerator4`
                (if (not (`self.HerbeIn?`))
                  (`StaticMeshComponent.SetStaticMesh` (`self.Slot3`) _interactitem_itemmesh)
                  (set `self.HerbeIn?` true)
                  (goto _label)
                  (else
                    (goto _label_2)))))
            (else
              (goto _label_2)))))
      (else
        (set `self.Interactable?` true)))))

(fn `Get Item Enum`
  (params (ItameRowName :type Name))
  (returns (`Finded?1` :type Boolean) (ItemEnum1 :type "/Game/SurvivalHorror1/Blueprints/Items_Inventory/All_Items Enum"))
  (locals (`Finded?` :type Boolean) (ItemEnum :type "/Game/SurvivalHorror1/Blueprints/Items_Inventory/All_Items Enum"))
  (bind _enumvalue (foreach `/Game/SurvivalHorror1/Blueprints/Items_Inventory/All_Items` false)
    (:`LoopBody`
      (if (== ItameRowName (`|GetEnumeratorNameAsString` _enumvalue))
        (set `local.Finded?` true)
        (set `local.ItemEnum` _enumvalue)))
    (:`then`
      (return (`local.Finded?`) (`local.ItemEnum`)))))

(fn `UserConstructionScript`)