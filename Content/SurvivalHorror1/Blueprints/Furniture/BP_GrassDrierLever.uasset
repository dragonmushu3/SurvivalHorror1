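; BP_GrassDrierLever is an interactable lever for the grass drier, usable only through its lever mesh and requiring no item.
; Interacting while enabled locks the lever, sends the player and itself to the first BP_GrassDrierCart found in the level, and plays a timeline that pitches the mesh.
; ToggleOff re-enables interaction and reverses the timeline to swing the lever back.
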(event `/Game/SurvivalHorror1/Blueprints/Main_Character/BPI_Interact.Interact`
  (params (Player :type "/Game/SurvivalHorror1/Blueprints/Main_Character/BP_MainCharacter Object Reference") (Component :type "ActorComponent Object Reference"))
  (set `self.Player` Player)
  (if (== Component (`self.SM_Levier`))
    (if (`self.Interactabled?`)
      (set `self.Interactabled?` false)
      (bind _outactors (`GameplayStatics.GetAllActorsOfClass` "/Game/SurvivalHorror1/Blueprints/Furniture/BP_GrassDrierCart.BP_GrassDrierCart_C"))
      (message `/Game/SurvivalHorror1/Blueprints/Furniture/BPI_GrassDrierCom.SendLeverData` (`|GetArrayItem` _outactors) (`self.Player`) self)
      (bind (_direction _lever) (`Timeline|Timeline` :!via `PlayFromStart` :!label _label)
        (:`Update`
          (`SceneComponent.K2_SetRelativeRotation` (`self.SM_Levier`) (`KismetMathLibrary.MakeRotator` 0.0 (`KismetMathLibrary.Lerp` 0.0 30.0 _lever)) false false))))))

(event `ToggleOff`
  (set `self.Interactabled?` true)
  (goto _label :!via `ReverseFromEnd`))

(fn `RequestInteractible?`
  (params (Component :type "ActorComponent Object Reference"))
  (returns (Interactable :type Boolean) (`NeedItem?` :type Boolean))
  (return (== Component (`self.SM_Levier`)) false))

(fn `UserConstructionScript`)