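; BP_WineFuserOut is the output side of a wine fuser that combines bottle, wine and herb into a DoorBottle item.
; SendWineInfo caches the player and WineInput references; when all three ingredient flags are set, it clears the input slot meshes, shows the final mesh and enables interaction.
; Interact adds DoorBottle to the player's inventory, clears the final mesh, and resets the flags on both itself and WineInput.
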(event `/Game/SurvivalHorror1/Blueprints/Furniture/BPI_WineCom.SendWineInfo`
  (params (Player :type "/Game/SurvivalHorror1/Blueprints/Main_Character/BP_MainCharacter Object Reference") (WineInput :type "/Game/SurvivalHorror1/Blueprints/Furniture/BP_WineFuser Object Reference"))
  (bind _wine_input (`self.Wine Input`))
  (set `self.Player` Player)
  (bind _output_get (set `self.Wine Input` WineInput))
  (set `self.BottleIn?` (`/Game/SurvivalHorror1/Blueprints/Furniture/BP_WineFuser.BottleIn?` _output_get))
  (set `self.WineIn?` (`/Game/SurvivalHorror1/Blueprints/Furniture/BP_WineFuser.WineIn?` _output_get))
  (set `self.HerbeIn?` (`/Game/SurvivalHorror1/Blueprints/Furniture/BP_WineFuser.HerbeIn?` _output_get))
  (if (and (`self.BottleIn?`) (`self.WineIn?`) (`self.HerbeIn?`))
    (`StaticMeshComponent.SetStaticMesh` (`/Game/SurvivalHorror1/Blueprints/Furniture/BP_WineFuser.Slot1` _wine_input) null)
    (`StaticMeshComponent.SetStaticMesh` (`/Game/SurvivalHorror1/Blueprints/Furniture/BP_WineFuser.Slot2` _wine_input) null)
    (`StaticMeshComponent.SetStaticMesh` (`/Game/SurvivalHorror1/Blueprints/Furniture/BP_WineFuser.Slot3` _wine_input) null)
    (`StaticMeshComponent.SetStaticMesh` (`self.SlotFinal`) "/Game/SurvivalHorror1/Art/LV1DiningQuarters/Bottles/LV1DiningQuarters_Walls_WB5.LV1DiningQuarters_Walls_WB5")
    (set `self.Interactable?` true)
    (else
      (set `self.Interactable?` false))))

(event `/Game/SurvivalHorror1/Blueprints/Main_Character/BPI_Interact.Interact`
  (params (Player :type "/Game/SurvivalHorror1/Blueprints/Main_Character/BP_MainCharacter Object Reference"))
  (bind _wine_input (`self.Wine Input`))
  (if (`self.Interactable?`)
    (`/Game/SurvivalHorror1/Blueprints/Inventory_V2/Comp_Inventory.AddToInventory` (`/Game/SurvivalHorror1/Blueprints/Main_Character/BP_MainCharacter.Comp_Inventory` (`self.Player`)) (`self.Door Bottle`))
    (`StaticMeshComponent.SetStaticMesh` (`self.SlotFinal`) null)
    (set `self.BottleIn?` false)
    (set `self.WineIn?` false)
    (set `self.HerbeIn?` false)
    (set `self.Interactable?` false)
    (set `/Game/SurvivalHorror1/Blueprints/Furniture/BP_WineFuser.BottleIn?` false _wine_input)
    (set `/Game/SurvivalHorror1/Blueprints/Furniture/BP_WineFuser.WineIn?` false _wine_input)
    (set `/Game/SurvivalHorror1/Blueprints/Furniture/BP_WineFuser.HerbeIn?` false _wine_input)))

(fn `UserConstructionScript`)