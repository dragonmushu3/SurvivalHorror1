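; Interactable alembic that turns wine, grass extract and an empty bottle into Fused Wine.
; The entry component takes wine and extract, returning their empty containers, while the stool or output slot takes the bottle and later gives the product.
; Once filled, PlayAnim locks it for a short delay, then shows the product mesh.
; Held items are identified by matching World_Items row names to an enum, and RequestInteractible reports per-component availability.
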(event `PlayAnim`
  (set `self.Interactable?` false)
  (`KismetSystemLibrary.RetriggerableDelay` 5.0)
  (bind _returnvalue (`|GetDataTableRow` "/Game/SurvivalHorror1/Blueprints/Items_Inventory/World_Items.World_Items" "Fused_wine")
    (:`then`
      (`StaticMeshComponent.SetStaticMesh` (`self.outItem`) (`.ItemMesh_25_1BE5031B4DE7578DCFA54481A5C4BD8D` (break `/Game/SurvivalHorror1/Blueprints/Items_Inventory/ST_Items` _returnvalue))))
    (:`RowNotFound`
      _))
  (set `self.GrassExtractIn?` false)
  (set `self.WineIn?` false)
  (set `self.EmptyBottleIn?` false)
  (set `self.FusedWineReady?` true)
  (set `self.Interactable?` true))

(event `/Game/SurvivalHorror1/Blueprints/Main_Character/BPI_Interact.Interact`
  (params (Player :type "/Game/SurvivalHorror1/Blueprints/Main_Character/BP_MainCharacter Object Reference") (Component :type "ActorComponent Object Reference"))
  (bind _item_equiped (`self.Item Equiped`))
  (bind _output_get (set `self.Player` Player))
  (set `self.Item Equiped` (`/Game/SurvivalHorror1/Blueprints/Items_Inventory/BP_InventoryManager.ItemEquiped` (`/Game/SurvivalHorror1/Blueprints/Main_Character/BP_MainCharacter.BP_InventoryManager` _output_get)))
  (set `self.Component` Component)
  (if (== (`self.Component`) (`self.outItem`))
    (if (`self.Interactable?`) :!label _label
      (if (not (`self.FusedWineReady?`))
        (if (not (`self.EmptyBottleIn?`))
          (bind _itemrowname (`self.getItemRowName` (`.ItemName_13_3536A9694BC1016CF006F3BFC8AE3C0B` (break `/Game/SurvivalHorror1/Blueprints/Items_Inventory/ST_Items` (`self.Item Equiped`))))
            (:`execout`
              (bind (_finded_1 _itemenum1) (`self.Get Item Enum` _itemrowname))
              (if _finded_1
                (set `self.Item Enum 1` _itemenum1)
                (if (`|EnumEquality` (`self.Item Enum 1`) "NewEnumerator0")
                  (bind _removed_ (`/Game/SurvivalHorror1/Blueprints/Items_Inventory/BP_InventoryManager.RemoveFromInventory` (`/Game/SurvivalHorror1/Blueprints/Main_Character/BP_MainCharacter.BP_InventoryManager` (`self.Player`)) _item_equiped))
                  (if _removed_
                    (set `self.EmptyBottleIn?` true)
                    (`StaticMeshComponent.SetStaticMesh` (`self.OutItem`) (`.ItemMesh_25_1BE5031B4DE7578DCFA54481A5C4BD8D` (break `/Game/SurvivalHorror1/Blueprints/Items_Inventory/ST_Items` _item_equiped)))
                    (if (and (`self.WineIn?`) (`self.EmptyBottleIn?`) (`self.GrassExtractIn?`)) :!label _label_2
                      (`self.PlayAnim`))
                    (else
                      (`KismetSystemLibrary.PrintString` "You need a bottle")))
                  (else
                    (`KismetSystemLibrary.PrintString` "You need a bottle in your hand")))
                (else
                  (`KismetSystemLibrary.PrintString` "No item in hand")))))
          (else
            (`KismetSystemLibrary.PrintString` "Empty bottle already in")))
        (else
          (bind _returnvalue (`|GetDataTableRow` "/Game/SurvivalHorror1/Blueprints/Items_Inventory/World_Items.World_Items" "Fused_wine")
            (:`then`
              (bind _added (`/Game/SurvivalHorror1/Blueprints/Items_Inventory/BP_InventoryManager.AddToInventory` (`/Game/SurvivalHorror1/Blueprints/Main_Character/BP_MainCharacter.BP_InventoryManager` (`self.Player`)) _returnvalue))
              (if _added
                (`StaticMeshComponent.SetStaticMesh` (`self.OutItem`) null)
                (set `self.FusedWineReady?` false)
                (else
                  (`KismetSystemLibrary.PrintString` "Inventorry full")))))))
      (else
        (`KismetSystemLibrary.PrintString` "Machine is doing something")))
    (elif (== (`self.Component`) (`self.SM_ExtractorStool`))
      (goto _label)
      (elif (== (`self.Component`) (`self.SM_AlambicEntry`))
        (if (`self.Interactable?`)
          (if (not (`self.FusedWineReady?`))
            (if (not (and (`self.GrassExtractIn?`) (`self.WineIn?`)))
              (`self.SetItemInHand`
                (:`ItemIn`
                  (if (`|EnumEquality` (`self.Item Enum 1`) "NewEnumerator17")
                    (bind _removed__2 (`/Game/SurvivalHorror1/Blueprints/Items_Inventory/BP_InventoryManager.RemoveFromInventory` (`/Game/SurvivalHorror1/Blueprints/Main_Character/BP_MainCharacter.BP_InventoryManager` (`self.Player`)) (`self.Item Equiped`)))
                    (if _removed__2
                      (set `self.GrassExtractIn?` true)
                      (bind _returnvalue_2 (`|GetDataTableRow` "/Game/SurvivalHorror1/Blueprints/Items_Inventory/World_Items.World_Items" "Flask_empty")
                        (:`then`
                          (bind _added_2 (`/Game/SurvivalHorror1/Blueprints/Items_Inventory/BP_InventoryManager.AddToInventory` (`/Game/SurvivalHorror1/Blueprints/Main_Character/BP_MainCharacter.BP_InventoryManager` (`self.Player`)) _returnvalue_2))
                          (if _added_2
                            (goto _label_2)
                            (else
                              (`KismetSystemLibrary.PrintString` "Inventorry full")))))
                      (else
                        (`KismetSystemLibrary.PrintString` "You need some grass extract")))
                    (elif (`|EnumEquality` (`self.Item Enum 1`) "NewEnumerator1")
                      (bind _removed__3 (`/Game/SurvivalHorror1/Blueprints/Items_Inventory/BP_InventoryManager.RemoveFromInventory` (`/Game/SurvivalHorror1/Blueprints/Main_Character/BP_MainCharacter.BP_InventoryManager` (`self.Player`)) (`self.Item Equiped`)))
                      (if _removed__3
                        (set `self.WineIn?` true)
                        (bind _returnvalue_3 (`|GetDataTableRow` "/Game/SurvivalHorror1/Blueprints/Items_Inventory/World_Items.World_Items" "Bottle_empty")
                          (:`then`
                            (bind _added_3 (`/Game/SurvivalHorror1/Blueprints/Items_Inventory/BP_InventoryManager.AddToInventory` (`/Game/SurvivalHorror1/Blueprints/Main_Character/BP_MainCharacter.BP_InventoryManager` (`self.Player`)) _returnvalue_3))
                            (if _added_3
                              (goto _label_2)
                              (else
                                (`KismetSystemLibrary.PrintString` "Inventorry full")))))
                        (else
                          (`KismetSystemLibrary.PrintString` "You need a Wine bottle")))
                      (elif (`self.WineIn?`)
                        (`KismetSystemLibrary.PrintString` "Wine already in")
                        (elif (`self.GrassExtractIn?`)
                          (`KismetSystemLibrary.PrintString` "Grass extract already in")
                          (else
                            (`KismetSystemLibrary.PrintString` "We don't need that here"))))))))
              (else
                (`KismetSystemLibrary.PrintString` "Grass extarct and Wine already in")))
            (else
              (`KismetSystemLibrary.PrintString` "Fused wine ready, pick it up")))
          (else
            (`KismetSystemLibrary.PrintString` "Machine is doing something")))))))

(fn `Get Item Enum`
  (params (ItameRowName :type Name))
  (returns (`Finded?1` :type Boolean) (ItemEnum1 :type "/Game/SurvivalHorror1/Blueprints/Items_Inventory/All_Items Enum"))
  (locals (`Finded?` :type Boolean) (ItemEnum :type "/Game/SurvivalHorror1/Blueprints/Items_Inventory/All_Items Enum"))
  (set `local.Finded?` false)
  (bind _enumvalue (foreach `/Game/SurvivalHorror1/Blueprints/Items_Inventory/All_Items` false)
    (:`LoopBody`
      (if (== ItameRowName (`|GetEnumeratorNameAsString` _enumvalue))
        (set `local.Finded?` true)
        (set `local.ItemEnum` _enumvalue)))
    (:`then`
      (return (`local.Finded?`) (`local.ItemEnum`)))))

(fn `RequestInteractible?`
  (params (Component :type "ActorComponent Object Reference"))
  (returns (Interactable :type Boolean) (`NeedItem?` :type Boolean))
  (bind _interactable_ (`self.Interactable?`))
  (bind _returnvalue (or (== Component (`self.SM_ExtractorStool`)) (== Component (`self.outItem`))))
  (bind _returnvalue_2 (and _returnvalue (not (`self.EmptyBottleIn?`))))
  (bind _returnvalue_3 (and (== Component (`self.SM_AlambicEntry`)) (or (not (`self.WineIn?`)) (not (`self.GrassExtractIn?`))) (not (`self.FusedWineReady?`))))
  (return (and (or _returnvalue_2 (and _returnvalue (`self.FusedWineReady?`)) _returnvalue_3) _interactable_) (and _interactable_ (or _returnvalue_2 _returnvalue_3))))

(fn `UserConstructionScript`)