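; Interactable furniture machine that turns dried grass and a flask from the player's inventory into grass extract.
; Interact routes by clicked component: plate takes grass, stool or output takes the flask or returns extract, and lever starts processing.
; A timeline animates door, hammer, lever and gear, then shows the extract mesh from the World_Items table.
; Equipped items are identified by matching data table row names to an enum, and RequestInteractible reports valid interactions.
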(event `PlayAnim`
  (set `self.Interactable?` false)
  (bind (_direction _doorrotation _hammerrotation) (`Timeline|Process` :!via `PlayFromStart`)
    (:`Update`
      (`SceneComponent.K2_SetRelativeRotation` (`self.door`) (`KismetMathLibrary.MakeRotator` 0.0 0.0 (`KismetMathLibrary.Lerp` 0.0 -135.0 _doorrotation)) false false)
      (bind _returnvalue (`KismetMathLibrary.Lerp` 0.0 -180.0 _hammerrotation))
      (`SceneComponent.K2_SetRelativeLocationAndRotation` (`self.SM_ExtractorHammer`) (`KismetMathLibrary.MakeVector` 0.0 0.0 (`KismetMathLibrary.Lerp` 0.0 -48.0 _hammerrotation)) (`KismetMathLibrary.MakeRotator` 0.0 0.0 _returnvalue) false false)
      (`SceneComponent.K2_SetRelativeRotation` (`self.lever`) (`KismetMathLibrary.MakeRotator` _returnvalue 0.0 -146.0) false false)
      (`SceneComponent.K2_SetRelativeRotation` (`self.SM_ExtractorEngrenage`) (`KismetMathLibrary.MakeRotator` 0.0 0.0 (`KismetMathLibrary.Lerp` 0.0 180.0 _hammerrotation)) false false))
    (:`Finished`
      (bind _returnvalue_2 (`|GetDataTableRow` "/Game/SurvivalHorror1/Blueprints/Items_Inventory/World_Items.World_Items" "Grass_extract")
        (:`then`
          (`StaticMeshComponent.SetStaticMesh` (`self.OutItem`) (`.ItemMesh_25_1BE5031B4DE7578DCFA54481A5C4BD8D` (break `/Game/SurvivalHorror1/Blueprints/Items_Inventory/ST_Items` _returnvalue_2))))
        (:`RowNotFound`
          _))
      (`StaticMeshComponent.SetStaticMesh` (`self.InItem`) null)
      (set `self.FioleIn?` false)
      (set `self.GrassIn` false)
      (set `self.ExtractReady?` true)
      (set `self.Interactable?` true))))

(event `/Game/SurvivalHorror1/Blueprints/Main_Character/BPI_Interact.Interact`
  (params (Player :type "/Game/SurvivalHorror1/Blueprints/Main_Character/BP_MainCharacter Object Reference") (Component :type "ActorComponent Object Reference"))
  (bind _item_equiped (`self.Item Equiped`))
  (bind _item_equiped_2 (`self.Item Equiped`))
  (bind _output_get (set `self.Player` Player))
  (set `self.Item Equiped` (`/Game/SurvivalHorror1/Blueprints/Items_Inventory/BP_InventoryManager.ItemEquiped` (`/Game/SurvivalHorror1/Blueprints/Main_Character/BP_MainCharacter.BP_InventoryManager` _output_get)))
  (set `self.Component` Component)
  (if (== (`self.Component`) (`self.SM_ExtractorLevel`))
    (if (`self.Interactable?`)
      (if (not (`self.ExtractReady?`))
        (if (and (`self.GrassIn`) (`self.FioleIn?`))
          (`self.PlayAnim`)
          (else
            (`KismetSystemLibrary.PrintString` "You need some dried grass and a flask")))
        (else
          (`KismetSystemLibrary.PrintString` "Grass extract ready, pick it up")))
      (else
        (`KismetSystemLibrary.PrintString` "Machine is doing something")))
    (elif (== (`self.Component`) (`self.OutItem`))
      (if (`self.Interactable?`) :!label _label
        (if (not (`self.ExtractReady?`))
          (if (not (`self.FioleIn?`))
            (bind _itemrowname (`self.getItemRowName` (`.ItemName_13_3536A9694BC1016CF006F3BFC8AE3C0B` (break `/Game/SurvivalHorror1/Blueprints/Items_Inventory/ST_Items` (`self.Item Equiped`))))
              (:`execout`
                (bind (_finded_1 _itemenum1) (`self.Get Item Enum` _itemrowname))
                (if _finded_1
                  (set `self.Item Enum 1` _itemenum1)
                  (if (`|EnumEquality` (`self.Item Enum 1`) "NewEnumerator18")
                    (bind _removed_ (`/Game/SurvivalHorror1/Blueprints/Items_Inventory/BP_InventoryManager.RemoveFromInventory` (`/Game/SurvivalHorror1/Blueprints/Main_Character/BP_MainCharacter.BP_InventoryManager` (`self.Player`)) _item_equiped_2))
                    (if _removed_
                      (set `self.FioleIn?` true)
                      (`StaticMeshComponent.SetStaticMesh` (`self.OutItem`) (`.ItemMesh_25_1BE5031B4DE7578DCFA54481A5C4BD8D` (break `/Game/SurvivalHorror1/Blueprints/Items_Inventory/ST_Items` _item_equiped_2)))
                      (else
                        (`KismetSystemLibrary.PrintString` "You need a flask")))
                    (else
                      (`KismetSystemLibrary.PrintString` "You need a flask in your hand")))
                  (else
                    (`KismetSystemLibrary.PrintString` "No item in hand")))))
            (else
              (`KismetSystemLibrary.PrintString` "Flask already in")))
          (else
            (bind _returnvalue (`|GetDataTableRow` "/Game/SurvivalHorror1/Blueprints/Items_Inventory/World_Items.World_Items" "Grass_extract")
              (:`then`
                (bind _added (`/Game/SurvivalHorror1/Blueprints/Items_Inventory/BP_InventoryManager.AddToInventory` (`/Game/SurvivalHorror1/Blueprints/Main_Character/BP_MainCharacter.BP_InventoryManager` (`self.Player`)) _returnvalue))
                (if _added
                  (`StaticMeshComponent.SetStaticMesh` (`self.OutItem`) null)
                  (set `self.ExtractReady?` false)
                  (else
                    (`KismetSystemLibrary.PrintString` "Inventorry full")))))))
        (else
          (`KismetSystemLibrary.PrintString` "Machine is doing something")))
      (elif (== (`self.Component`) (`self.SM_ExtractorStool`))
        (goto _label)
        (elif (== (`self.Component`) (`self.SM_ExtractorPlate`))
          (if (`self.Interactable?`)
            (if (not (`self.ExtractReady?`))
              (if (not (`self.GrassIn`))
                (bind _itemrowname_2 (`self.getItemRowName` (`.ItemName_13_3536A9694BC1016CF006F3BFC8AE3C0B` (break `/Game/SurvivalHorror1/Blueprints/Items_Inventory/ST_Items` (`self.Item Equiped`))))
                  (:`execout`
                    (bind (_finded_1_2 _itemenum1_2) (`self.Get Item Enum` _itemrowname_2))
                    (if _finded_1_2
                      (set `self.Item Enum 1` _itemenum1_2)
                      (if (`|EnumEquality` (`self.Item Enum 1`) "NewEnumerator16")
                        (bind _removed__2 (`/Game/SurvivalHorror1/Blueprints/Items_Inventory/BP_InventoryManager.RemoveFromInventory` (`/Game/SurvivalHorror1/Blueprints/Main_Character/BP_MainCharacter.BP_InventoryManager` (`self.Player`)) _item_equiped))
                        (if _removed__2
                          (set `self.GrassIn` true)
                          (`StaticMeshComponent.SetStaticMesh` (`self.InItem`) (`.ItemMesh_25_1BE5031B4DE7578DCFA54481A5C4BD8D` (break `/Game/SurvivalHorror1/Blueprints/Items_Inventory/ST_Items` _item_equiped)))
                          (else
                            (`KismetSystemLibrary.PrintString` "You need some dried grass")))
                        (else
                          (`KismetSystemLibrary.PrintString` "You need some dryed grass in your hand")))
                      (else
                        (`KismetSystemLibrary.PrintString` "No item in hand")))))
                (else
                  (`KismetSystemLibrary.PrintString` "Grass already in")))
              (else
                (`KismetSystemLibrary.PrintString` "Grass extract ready, pick it up")))
            (else
              (`KismetSystemLibrary.PrintString` "Machine is doing something"))))))))

(fn `Get Item Enum`
  (params (ItameRowName :type Name))
  (returns (`Finded?1` :type Boolean) (ItemEnum1 :type "/Game/SurvivalHorror1/Blueprints/Items_Inventory/All_Items Enum"))
  (locals (`Finded?` :type Boolean) (ItemEnum :type "/Game/SurvivalHorror1/Blueprints/Items_Inventory/All_Items Enum"))
  (set `local.Finded?` false)
  (bind _enumvalue (foreach `/Game/SurvivalHorror1/Blueprints/Items_Inventory/All_Items` false)
    (:`LoopBody`
      (if (== ItameRowName (`|GetEnumeratorNameAsString` _enumvalue))
        (set `local.Finded?` true)
        (set `local.ItemEnum` _enumvalue)))
    (:`then`
      (return (`local.Finded?`) (`local.ItemEnum`)))))

(fn `RequestInteractible?`
  (params (Component :type "ActorComponent Object Reference"))
  (returns (Interactable :type Boolean) (`NeedItem?` :type Boolean))
  (bind _interactable_ (`self.Interactable?`))
  (bind _grassin (`self.GrassIn`))
  (bind _returnvalue (or (== Component (`self.OutItem`)) (== Component (`self.SM_ExtractorStool`))))
  (bind _returnvalue_2 (and (== Component (`self.SM_ExtractorPlate`)) (not _grassin) (not (`self.ExtractReady?`))))
  (bind _returnvalue_3 (and _returnvalue (not (`self.FioleIn?`))))
  (return (and (or (and (== Component (`self.SM_ExtractorLevel`)) (`self.FioleIn?`) _grassin) _returnvalue_2 _returnvalue_3 (and _returnvalue (`self.ExtractReady?`))) _interactable_) (and _interactable_ (or _returnvalue_2 _returnvalue_3))))

(fn `UserConstructionScript`)