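; BP_EndDoorOut is an end door furniture Blueprint that opens when it receives the SendEndDoorInfo event.
; The event plays a creaking door sound at the root's location and runs a timeline that lerps the EndDoor component's relative yaw to swing it open a quarter turn.
; A getInteractItem graph holds only an unused lookup of the last item in the player's inventory.
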(event `/Game/SurvivalHorror1/Blueprints/Furniture/BPI_EndDoorCom.SendEndDoorInfo`
  (params (Vase :type "/Game/SurvivalHorror1/Blueprints/Furniture/BP_EndDoor Object Reference"))
  (`GameplayStatics.PlaySoundAtLocation` "/Game/SurvivalHorror1/Sound/Effects/grincement_porte.grincement_porte" (`SceneComponent.K2_GetComponentLocation` (`self.DefaultSceneRoot`)) (struct) 1.0 1.0 0.0 null null null null)
  (bind (_direction _door) (`Timeline|Timeline` :!via `PlayFromStart`)
    (:`Update`
      (`SceneComponent.K2_SetRelativeRotation` (`self.EndDoor`) (`KismetMathLibrary.MakeRotator` 0.0 0.0 (`KismetMathLibrary.Lerp` 0.0 -90.0 _door)) false false))))

(fn `UserConstructionScript`)