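; Interactable wine machine furniture that turns an accepted equipped item into a full wine bottle for the player's inventory.
; Interact matches the item's World_Items row name to an item enum, shows its mesh in SlotHaut, removes it from inventory and becomes ready after a short delay.
; The next interaction grants the bottle and clears the slot.
; RequestInteractible reports interaction and item-need states, while IsBroken disables processing.
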(event `/Game/SurvivalHorror1/Blueprints/Main_Character/BPI_Interact.Interact`
  (params (Player :type "/Game/SurvivalHorror1/Blueprints/Main_Character/BP_MainCharacter Object Reference") (Component :type "ActorComponent Object Reference"))
  (bind (_itemname _itemtype _description _itemicon _itemmesh) (break `/Game/SurvivalHorror1/Blueprints/Items_Inventory/ST_Items` (`self.Item Equiped`)))
  (bind _output_get (set `self.Player` Player))
  (set `self.Item Equiped` (`/Game/SurvivalHorror1/Blueprints/Items_Inventory/BP_InventoryManager.ItemEquiped` (`/Game/SurvivalHorror1/Blueprints/Main_Character/BP_MainCharacter.BP_InventoryManager` _output_get)))
  (if (not (`self.IsBroken?`))
    (if (`self.Interactable?`)
      (if (not (`self.ItemReady?`))
        (set `self.Interactable?` false)
        (bind _itemrowname (`self.getItemRowName` _itemname)
          (:`execout`
            (bind (_finded_1 _itemenum1) (`self.Get Item Enum` _itemrowname))
            (if _finded_1
              (if (`|EnumEquality` _itemenum1 "NewEnumerator0")
                (`StaticMeshComponent.SetStaticMesh` (`self.slot_haut`) _itemmesh)
                (`/Game/SurvivalHorror1/Blueprints/Items_Inventory/BP_InventoryManager.RemoveFromInventory` (`/Game/SurvivalHorror1/Blueprints/Main_Character/BP_MainCharacter.BP_InventoryManager` (`self.Player`)) (`self.Item Equiped`))
                (`KismetSystemLibrary.RetriggerableDelay` 2.0)
                (set `self.Interactable?` true)
                (set `self.ItemReady?` true)
                (else
                  (set `self.Interactable?` true :!label _label)))
              (else
                (goto _label)))))
        (else
          (bind _returnvalue (`|GetDataTableRow` "/Game/SurvivalHorror1/Blueprints/Items_Inventory/World_Items.World_Items" "Wine_bottle_full")
            (:`then`
              (`/Game/SurvivalHorror1/Blueprints/Items_Inventory/BP_InventoryManager.AddToInventory` (`/Game/SurvivalHorror1/Blueprints/Main_Character/BP_MainCharacter.BP_InventoryManager` (`self.Player`)) _returnvalue)
              (`StaticMeshComponent.SetStaticMesh` (`self.slot_haut`) null)
              (set `self.ItemReady?` false)))))
      (else
        (set `self.Interactable?` true)))))

(fn `Get Item Enum`
  (params (ItameRowName :type Name))
  (returns (`Finded?1` :type Boolean) (ItemEnum1 :type "/Game/SurvivalHorror1/Blueprints/Items_Inventory/All_Items Enum"))
  (locals (`Finded?` :type Boolean) (ItemEnum :type "/Game/SurvivalHorror1/Blueprints/Items_Inventory/All_Items Enum"))
  (set `local.Finded?` false)
  (bind _enumvalue (foreach `/Game/SurvivalHorror1/Blueprints/Items_Inventory/All_Items` false)
    (:`LoopBody`
      (if (== ItameRowName (`|GetEnumeratorNameAsString` _enumvalue))
        (set `local.Finded?` true)
        (set `local.ItemEnum` _enumvalue)))
    (:`then`
      (return (`local.Finded?`) (`local.ItemEnum`)))))

(fn `RequestInteractible?`
  (params (Component :type "ActorComponent Object Reference"))
  (returns (Interactable :type Boolean) (`NeedItem?` :type Boolean))
  (bind _returnvalue (or (== Component (`self.étagère_haute`)) (== Component (`self.slot_haut`))))
  (bind _returnvalue_2 (and _returnvalue (`self.Interactable?`) (not (`self.ItemReady?`))))
  (return (or _returnvalue_2 (and _returnvalue (`self.ItemReady?`))) _returnvalue_2))

(fn `UserConstructionScript`
  (if (`self.IsBroken?`)
    (set `self.Interactable?` false)))