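; BP_EndDoor is an interactable end door that accepts the Bottle Door item from the player's inventory.
; On Interact, it matches the equipped item's name against the item enum.
; For Bottle Door, it removes the item and sends itself to the first BP_EndDoorOut via SendEndDoorInfoMessage.
; Interaction locks on use and re-enables only when no enum entry matches, so other recognized items also leave it locked.
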(event `/Game/SurvivalHorror1/Blueprints/Main_Character/BPI_Interact.Interact`
  (params (Player :type "/Game/SurvivalHorror1/Blueprints/Main_Character/BP_MainCharacter Object Reference"))
  (bind _item_equiped_itemname (break `/Game/SurvivalHorror1/Blueprints/Items_Inventory/ST_Items` (`self.Item Equiped`)))
  (bind _output_get (set `self.Player` Player))
  (set `self.Item Equiped` (`/Game/SurvivalHorror1/Blueprints/Items_Inventory/BP_InventoryManager.ItemEquiped` (`/Game/SurvivalHorror1/Blueprints/Main_Character/BP_MainCharacter.BP_InventoryManager` _output_get)))
  (if (`self.Interactable?`)
    (set `self.Interactable?` false)
    (bind (_finded_1 _itemenum1) (`self.Get Item Enum` _item_equiped_itemname))
    (if _finded_1
      (switch `/Game/SurvivalHorror1/Blueprints/Items_Inventory/All_Items` _itemenum1
        (:`NewEnumerator3`
          (`/Game/SurvivalHorror1/Blueprints/Items_Inventory/BP_InventoryManager.RemoveFromInventory` (`/Game/SurvivalHorror1/Blueprints/Main_Character/BP_MainCharacter.BP_InventoryManager` (`self.Player`)) (`self.Item Equiped`))
          (bind _outactors (`GameplayStatics.GetAllActorsOfClass` "/Game/SurvivalHorror1/Blueprints/Furniture/BP_EndDoorOut.BP_EndDoorOut_C"))
          (message `/Game/SurvivalHorror1/Blueprints/Furniture/BPI_EndDoorCom.SendEndDoorInfo` (`|GetArrayItem` _outactors) self)))
      (else
        (set `self.Interactable?` true)))))

(fn `Get Item Enum`
  (params (ItameRowName :type Name))
  (returns (`Finded?1` :type Boolean) (ItemEnum1 :type "/Game/SurvivalHorror1/Blueprints/Items_Inventory/All_Items Enum"))
  (locals (`Finded?` :type Boolean) (ItemEnum :type "/Game/SurvivalHorror1/Blueprints/Items_Inventory/All_Items Enum"))
  (bind _enumvalue (foreach `/Game/SurvivalHorror1/Blueprints/Items_Inventory/All_Items` false)
    (:`LoopBody`
      (if (== ItameRowName (`|GetEnumeratorName` _enumvalue))
        (set `local.Finded?` true)
        (set `local.ItemEnum` _enumvalue)))
    (:`then`
      (return (`local.Finded?`) (`local.ItemEnum`)))))

(fn `UserConstructionScript`)