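; BP_Melangeur is an interactible mixer that turns fused wine into a Bottle_Door item.
; Interacting with the body loads the equipped item after a name-to-row-to-enum check, or hands over the finished bottle through the player's inventory manager.
; Interacting with the stick calls PlayAnim, which converts instantly because the Mixing timeline animation is never triggered.
; RequestInteractible reports whether each component is usable or needs an item.
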(event `Play Anim`
  (set `self.FusedWineIn?` false)
  (set `self.BottleDoorReady?` true))

(event `/Game/SurvivalHorror1/Blueprints/Main_Character/BPI_Interact.Interact`
  (params (Player :type "/Game/SurvivalHorror1/Blueprints/Main_Character/BP_MainCharacter Object Reference") (Component :type "ActorComponent Object Reference"))
  (bind _output_get (set `self.Player` Player))
  (set `self.Item Equiped` (`/Game/SurvivalHorror1/Blueprints/Items_Inventory/BP_InventoryManager.ItemEquiped` (`/Game/SurvivalHorror1/Blueprints/Main_Character/BP_MainCharacter.BP_InventoryManager` _output_get)))
  (set `self.Component` Component)
  (if (== (`self.Component`) (`self.SM_MelangeurBaton`))
    (if (`self.Interactible?`)
      (if (not (`self.BottleDoorReady?`))
        (if (`self.FusedWineIn?`)
          (`self.Play Anim`)
          (else
            (`KismetSystemLibrary.PrintString` "You need a bottle of fused wine")))
        (else
          (`KismetSystemLibrary.PrintString` "Door bottle ready, pick it up")))
      (else
        (`KismetSystemLibrary.PrintString` "Machine is doing something")))
    (elif (== (`self.Component`) (`self.SM_Melangeur`))
      (if (`self.Interactible?`)
        (if (not (`self.BottleDoorReady?`))
          (if (not (`self.FusedWineIn?`))
            (bind _itemrowname (`self.getItemRowName` (`.ItemName_13_3536A9694BC1016CF006F3BFC8AE3C0B` (break `/Game/SurvivalHorror1/Blueprints/Items_Inventory/ST_Items` (`self.Item Equiped`))))
              (:`execout`
                (bind (_finded_1 _itemenum1) (`self.Get Item Enum` _itemrowname))
                (if _finded_1
                  (set `self.Item Enum 1` _itemenum1)
                  (if (`|EnumEquality` (`self.Item Enum 1`) "NewEnumerator2")
                    (bind _removed_ (`/Game/SurvivalHorror1/Blueprints/Items_Inventory/BP_InventoryManager.RemoveFromInventory` (`/Game/SurvivalHorror1/Blueprints/Main_Character/BP_MainCharacter.BP_InventoryManager` (`self.Player`)) (`self.Item Equiped`)))
                    (if _removed_
                      (set `self.FusedWineIn?` true)
                      (else
                        (`KismetSystemLibrary.PrintString` "You need a bottle of fused wine")))
                    (else
                      (`KismetSystemLibrary.PrintString` "You need a bottle of fused wine in your hand")))
                  (else
                    (`KismetSystemLibrary.PrintString` "No item in hand")))))
            (else
              (`KismetSystemLibrary.PrintString` "Fused Wine already in")))
          (else
            (bind _returnvalue (`|GetDataTableRow` "/Game/SurvivalHorror1/Blueprints/Items_Inventory/World_Items.World_Items" "Bottle_Door")
              (:`then`
                (bind _added (`/Game/SurvivalHorror1/Blueprints/Items_Inventory/BP_InventoryManager.AddToInventory` (`/Game/SurvivalHorror1/Blueprints/Main_Character/BP_MainCharacter.BP_InventoryManager` (`self.Player`)) _returnvalue))
                (if _added
                  (set `self.BottleDoorReady?` false)
                  (else
                    (`KismetSystemLibrary.PrintString` "Inventorry full")))))))
        (else
          (`KismetSystemLibrary.PrintString` "Machine is doing something"))))))

(fn `Get Item Enum`
  (params (ItameRowName :type Name))
  (returns (`Finded?1` :type Boolean) (ItemEnum1 :type "/Game/SurvivalHorror1/Blueprints/Items_Inventory/All_Items Enum"))
  (locals (`Finded?` :type Boolean) (ItemEnum :type "/Game/SurvivalHorror1/Blueprints/Items_Inventory/All_Items Enum"))
  (set `local.Finded?` false)
  (bind _enumvalue (foreach `/Game/SurvivalHorror1/Blueprints/Items_Inventory/All_Items` false)
    (:`LoopBody`
      (if (== ItameRowName (`|GetEnumeratorNameAsString` _enumvalue))
        (set `local.Finded?` true)
        (set `local.ItemEnum` _enumvalue)))
    (:`then`
      (return (`local.Finded?`) (`local.ItemEnum`)))))

(fn `RequestInteractible?`
  (params (Component :type "ActorComponent Object Reference"))
  (returns (Interactable :type Boolean) (`NeedItem?` :type Boolean))
  (bind _interactible_ (`self.Interactible?`))
  (bind _returnvalue (== Component (`self.SM_Melangeur`)))
  (bind _returnvalue_2 (and _returnvalue (not (`self.FusedWineIn?`)) (not (`self.BottleDoorReady?`))))
  (return (and (or (and (== Component (`self.SM_MelangeurBaton`)) (`self.FusedWineIn?`)) _returnvalue_2 (and _returnvalue (`self.BottleDoorReady?`))) _interactible_) (and _returnvalue_2 _interactible_)))

(fn `UserConstructionScript`)